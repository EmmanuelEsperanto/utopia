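; Base ghost for building parts in the survival pack's build system, extending the parent ghost's placement logic.
; The condition pass defers to the parent check, and rotation, when locked, converts current yaw into mode-selected steps added to the socket's yaw, otherwise using the current rotation.
; Socket-location getters for foundations, floors, walls, roofs, ground and special snaps are empty here, apparently for child parts to override, and the part type returns a default enum.
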(fn ConstructionScript
  (|CallParentFunction))

(fn CustomConditionPass
  (params (Hit :type Hit%20Result%20Structure) (Locked%20Location :type Boolean))
  (bind _return (|CallParentFunction Hit Locked%20Location)) ; Is Build Type = Building?
  (if _return
    (return true)
    (else
      (return false))))

(fn CustomRotation
  (params (Hit :type Hit%20Result%20Structure) (Current%20Rotation :type Rotator :default "0, 0, 0") (Socket%20Rotation :type Rotator :default "0, 0, 0") (Locked%20Location :type Boolean) (Rotation%20Mode :type E_RotationMode%20Enum :default "NewEnumerator0"))
  (if Locked%20Location
    (Transformation|SetActorRotation (Math|Rotator|MakeRotator 0.0 0.0 (+ (* (/ (.yaw Current%20Rotation) 15.0) (Utilities|Select :Index Rotation%20Mode :NewEnumerator0 9e+01 :NewEnumerator1 1.8e+02 :NewEnumerator2 0.0)) (.Yaw (Math|Rotator|BreakRotator Socket%20Rotation)))))
    (else
      (Transformation|SetActorRotation (Math|Rotator|MakeRotator (.roll Current%20Rotation) (.pitch Current%20Rotation) (.yaw Current%20Rotation))))))

(fn GetAngledFloorLocations
  (return 0))

(fn GetAngledFoundationLocations
  (return 0))

(fn GetFloorLocations
  (return 0))

(fn GetFoundationLocations
  (return 0))

(fn GetGroundLocations
  (return 0))

(fn GetPartType
  (return "NewEnumerator0"))

(fn GetRoofLocations
  (return 0))

(fn GetSpecialLocations
  (return 0))

(fn GetWallLocations
  (return 0))