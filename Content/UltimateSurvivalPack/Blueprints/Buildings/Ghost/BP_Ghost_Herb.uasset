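; BP_Ghost_Herb is a building ghost for placing a herb in the survival pack.
; Its custom condition pass succeeds only when the hit surface faces nearly straight up and the hit actor's class is BP_Planter or BP_SmallPlanter.
; Its vector modification ignores the input and returns a zero vector, while the construction script just calls the parent.
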(fn ConstructionScript
  (|CallParentFunction))

(fn CustomConditionPass
  (params (Hit :type Hit%20Result%20Structure) (Locked%20Location :type Boolean))
  (bind (_bblockinghit _binitialoverlap _time _distance _location _impactpoint _normal _impactnormal _physmat _hitactor) (Collision|BreakHitResult Hit))
  (return (and (> (.Z (Math|Vector|BreakVector _impactnormal)) 0.9) (Utilities|Array|ContainsItem (Utilities|Array|MakeArray "/Game/UltimateSurvivalPack/Blueprints/Buildings/Final/BP_Planter.BP_Planter_C" "/Game/UltimateSurvivalPack/Blueprints/Buildings/Final/BP_SmallPlanter.BP_SmallPlanter_C") (Utilities|GetClass _hitactor)))))

(fn VectorModification
  (params (Vector :type Vector :default "0, 0, 0"))
  (return "0, 0, 0"))