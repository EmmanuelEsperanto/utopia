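; BP_Ghost_Carpet is the building ghost for a carpet, with rules for where it can be placed.
; Its condition check passes only when the hit actor has a BP_BuildingComponent of one specific build type and the surface normal points mostly upward.
; Its vector modification returns zero regardless of input, and construction defers to the parent.
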(fn ConstructionScript
  (|CallParentFunction))

(fn CustomConditionPass
  (params (Hit :type Hit%20Result%20Structure) (Locked%20Location :type Boolean))
  (bind _hitactor (Collision|BreakHitResult Hit))
  (bind _returnvalue (Actor|GetComponentbyClass _hitactor "/Game/UltimateSurvivalPack/Blueprints/Buildings/Parent/BP_BuildingComponent.BP_BuildingComponent_C"))
  (Utilities|IsValid _returnvalue
    (:Is%20Valid
      (if (Utilities|Enum|Equal(Enum) (.BuildType (Utilities|Struct|BreakS_Building (Variables|/Game/UltimateSurvivalPack/Blueprints/Buildings/Parent/BP_BuildingComponent.BP_BuildingComponent_C|GetBuild%20Data _returnvalue))) "NewEnumerator0")
        (return (> (.Z (Math|Vector|BreakVector (.ImpactNormal (Collision|BreakHitResult Hit)))) 0.75))
        (else
          _)))
    (:Is%20Not%20Valid
      _))
  (return false))

(fn VectorModification
  (params (Vector :type Vector :default "0, 0, 0"))
  (return "0, 0, 0"))