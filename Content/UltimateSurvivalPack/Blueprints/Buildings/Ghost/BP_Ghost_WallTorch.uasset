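; Placement ghost for a wall torch in the building system, extending a parent ghost through overridden placement hooks.
; Placement passes only if the parent check succeeds and the hit surface is roughly vertical, judged by the impact normal's Z.
; Custom rotation turns the ghost's X axis along the surface normal so it faces out from the wall.
; The vector modification hook always returns a zero vector.
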(fn ConstructionScript
  (|CallParentFunction))

(fn CustomConditionPass
  (params (Hit :type Hit%20Result%20Structure) (Locked%20Location :type Boolean))
  (bind _return (|CallParentFunction Hit false)) ; Is Build Type = Building?
  (if _return
    (return (Math|Float|NearlyEqual(Float) (.Z (Math|Vector|BreakVector (.ImpactNormal (Collision|BreakHitResult Hit)))) 0.0 0.4))
    (else
      (return false))))

(fn CustomRotation
  (params (Hit :type Hit%20Result%20Structure) (Current%20Rotation :type Rotator :default "0, 0, 0") (Socket%20Rotation :type Rotator :default "0, 0, 0") (Locked%20Location :type Boolean) (Rotation%20Mode :type E_RotationMode%20Enum :default "NewEnumerator0"))
  (Transformation|SetActorRotation (Math|Rotator|MakeRotfromX (.ImpactNormal (Collision|BreakHitResult Hit))))
  (return))

(fn VectorModification
  (params (Vector :type Vector :default "0, 0, 0"))
  (return "0, 0, 0"))