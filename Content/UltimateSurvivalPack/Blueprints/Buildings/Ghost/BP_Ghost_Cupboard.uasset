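; Placement ghost for the cupboard in the building system, deciding whether the previewed cupboard may be placed.
; It extends the parent condition pass with a parental-cupboard check and requires a near-flat, upward-facing hit surface.
; A sphere trace around the ghost then rejects placement if another BP_Cupboard is within range, keeping cupboards spaced apart.
; The vector modification override always returns a zero vector.
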(fn ConstructionScript
  (|CallParentFunction))

(fn CustomConditionPass
  (params (Hit :type Hit%20Result%20Structure) (Locked%20Location :type Boolean))
  (bind _returnvalue (Transformation|GetActorLocation))
  (bind _return (|CallParentFunction Hit false)) ; Is Build Type = Building?
  (if _return
    (bind _return_2 (CallFunction|IsParentalCupboard))
    (if _return_2
      (if (> (.Z (Math|Vector|BreakVector (.ImpactNormal (Collision|BreakHitResult Hit)))) 0.9)
        (bind _outhits (Collision|MultiSphereTraceForObjects _returnvalue _returnvalue 1.5e+03 (Utilities|Array|MakeArray "ObjectTypeQuery2") false 0 "None"))
        (for _array_element _outhits
          (Utilities|Casting|CastToBP_Cupboard (.HitActor (Collision|BreakHitResult _array_element)))
          (return false))
        (return true))
      (else
        (return false)))
    (else
      (return false))))

(fn VectorModification
  (params (Vector :type Vector :default "0, 0, 0"))
  (return "0, 0, 0"))