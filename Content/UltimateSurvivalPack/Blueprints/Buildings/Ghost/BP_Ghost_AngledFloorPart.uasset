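; BP_Ghost_AngledFloorPart is the building placement ghost for an angled floor piece, overriding part type, placement check and rotation from its parent.
; Placement passes only when the parent condition succeeds and the location is locked.
; When locked, rotation converts each 15-degree yaw step into a 120-degree step added to the socket yaw.
; When unlocked, it uses the current rotation directly.
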(event EventBeginPlay)

(event Collision|EventActorBeginOverlap
  (params (OtherActor :type Actor%20Object%20Reference)))

(event EventTick
  (params (DeltaSeconds :type Float%20%28single-precision%29)))

(fn ConstructionScript
  (|CallParentFunction))

(fn GetPartType
  (return "NewEnumerator8"))

(fn CustomConditionPass
  (params (Hit :type Hit%20Result%20Structure) (Locked%20Location :type Boolean))
  (bind _return (|CallParentFunction Hit Locked%20Location))
  (return (and _return Locked%20Location)))

(fn CustomRotation
  (params (Hit :type Hit%20Result%20Structure) (Current%20Rotation :type Rotator :default "0, 0, 0") (Socket%20Rotation :type Rotator :default "0, 0, 0") (Locked%20Location :type Boolean) (Rotation%20Mode :type E_RotationMode%20Enum :default "NewEnumerator0"))
  (if Locked%20Location
    (Transformation|SetActorRotation (Math|Rotator|MakeRotator 0.0 0.0 (+ (* (/ (.yaw Current%20Rotation) 15.0) 1.2e+02) (.Yaw (Math|Rotator|BreakRotator Socket%20Rotation)))))
    (else
      (Transformation|SetActorRotation (Math|Rotator|MakeRotator (.roll Current%20Rotation) (.pitch Current%20Rotation) (.yaw Current%20Rotation)))))
  (return))