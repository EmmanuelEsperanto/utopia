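; Parent ghost actor for building placement, providing material feedback and the checks that decide whether a piece can be placed.
; SetGhostColor restores mesh materials or applies red, skipping components tagged Custom.
; CollisionCheck box-traces the BuildData volume in both directions, filtering hits by class, while cupboard traces find nearby cupboards and verify player privilege.
; Custom functions restrict build type, align rotation to the surface normal, allow location locking and clamp vector height.
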(fn ConstructionScript)

(fn SetGhostColor
  (params (Success :type Boolean))
  (if Success
    ;[0.3763 1 0.239] Set Normal Material
    (for _array_element (Actor|GetComponentsByClass "/Script/Engine.StaticMeshComponent")
      (if (not (Utilities|Array|ContainsItem (Variables|/Script/Engine.ActorComponent|GetComponentTags _array_element) "Custom"))
        (bind _staticmesh (Variables|/Script/Engine.StaticMeshComponent|GetStaticMesh _array_element)
          (:then
            (for (_array_element_2 _array_index) (Variables|/Script/Engine.StaticMesh|GetStaticMaterials _staticmesh)
              (Rendering|Material|SetMaterial _array_element _array_index (Utilities|Struct|BreakStaticMaterial _array_element_2))))
          (:else))))
    (else
      ;[1 0.1212 0.07146] Set Red Material
      (for _array_element_3 (Actor|GetComponentsByClass "/Script/Engine.StaticMeshComponent")
        (if (not (Utilities|Array|ContainsItem (Variables|/Script/Engine.ActorComponent|GetComponentTags _array_element_3) "Custom"))
          (bind _staticmesh_2 (Variables|/Script/Engine.StaticMeshComponent|GetStaticMesh _array_element_3)
            (:then
              (for (_ _array_index_2) (Variables|/Script/Engine.StaticMesh|GetStaticMaterials _staticmesh_2)
                (Rendering|Material|SetMaterial _array_element_3 _array_index_2 "/Game/UltimateSurvivalPack/Material/MI_Ghost_Red.MI_Ghost_Red")))
            (:else)))))))

(fn CustomConditionPass
  (params (Hit :type Hit%20Result%20Structure) (Locked%20Location :type Boolean))
  (bind _hitactor (Collision|BreakHitResult Hit))
  (bind _returnvalue (Actor|GetComponentbyClass _hitactor "/Game/UltimateSurvivalPack/Blueprints/Buildings/Parent/BP_BuildingComponent.BP_BuildingComponent_C"))
  ;[1 1 1] Only Place Building On Type = Building
  (Utilities|IsValid _returnvalue
    (:Is%20Valid
      (return (Utilities|Enum|Equal(Enum) (.BuildType (Utilities|Struct|BreakS_Building (Variables|/Game/UltimateSurvivalPack/Blueprints/Buildings/Parent/BP_BuildingComponent.BP_BuildingComponent_C|GetBuild%20Data _returnvalue))) "NewEnumerator0")))
    (:Is%20Not%20Valid
      (return true))))

(fn CustomRotation
  (params (Hit :type Hit%20Result%20Structure) (Current%20Rotation :type Rotator) (Socket%20Rotation :type Rotator) (Locked%20Location :type Boolean) (Rotation%20Mode :type E_RotationMode%20Enum :default "NewEnumerator0"))
  (bind _impactnormal (Collision|BreakHitResult Hit))
  (Transformation|SetActorRotation (Math|Rotator|CombineRotators (Math|Rotator|MakeRotator 0.0 0.0 (+ (.Yaw (Math|Rotator|BreakRotator Current%20Rotation)) (select (Class|KismetMathLibrary|EqualExactlyVectorVector _impactnormal "0, 0, 0") 0.0 9e+01))) (Math|Rotator|MakeRotfromZ _impactnormal)))
  (return))

(fn CollisionCheck
  (bind _returnvalue (Transformation|GetActorRotation))
  (bind _returnvalue_2 (Transformation|GetActorRotation))
  (bind _build_data (Variables|Default|GetBuild%20Data))
  (bind _build_data_2 (Variables|Default|GetBuild%20Data))
  (bind _collisiontransform (Utilities|Struct|BreakS_Building _build_data))
  (bind _collisiontransform_2 (Utilities|Struct|BreakS_Building _build_data_2))
  (bind (_roll _pitch _yaw) (Math|Rotator|BreakRotator _returnvalue_2))
  (bind (_roll_2 _pitch_2 _yaw_2) (Math|Rotator|BreakRotator _returnvalue))
  (bind (_location _rotation _scale) (Math|Transform|BreakTransform _collisiontransform))
  (bind (_location_2 _rotation_2 _scale_2) (Math|Transform|BreakTransform _collisiontransform_2))
  (bind _x (Math|Vector|BreakVector _scale))
  (bind (_x_2 _y _z) (Math|Vector|BreakVector _scale))
  (bind (_roll_3 _pitch_3 _yaw_3) (Math|Rotator|BreakRotator _rotation))
  (bind (_roll_4 _pitch_4 _yaw_4) (Math|Rotator|BreakRotator _rotation_2))
  (bind _x_3 (Math|Vector|BreakVector _scale_2))
  (bind (_x_4 _y_2 _z_2) (Math|Vector|BreakVector _scale_2))
  (bind (_outhits _returnvalue_3) (Class|KismetSystemLibrary|BoxTraceMultiforObjects (+ (Transformation|GetActorLocation) (Math|Vector|RotateVector (+ _location_2 (Math|Vector|MakeVector _x_3 0.0 0.0)) _returnvalue)) (+ (Transformation|GetActorLocation) (Math|Vector|RotateVector (- _location_2 (Math|Vector|MakeVector _x_3 0.0 0.0)) _returnvalue)) (Math|Vector|MakeVector 1.0 _y_2 _z_2) (Math|Rotator|MakeRotator (+ _roll_2 _roll_4) (+ _pitch_2 _pitch_4) (+ _yaw_2 _yaw_4)) (Utilities|Array|MakeArray "ObjectTypeQuery1" "ObjectTypeQuery3" "ObjectTypeQuery6" "ObjectTypeQuery5") false 0 "None" true))
  (if _returnvalue_3
    (bind _return (CallFunction|FilterCollisionHit _outhits))
    (if _return
      (bind (_outhits_2 _returnvalue_4) (Class|KismetSystemLibrary|BoxTraceMultiforObjects (+ (Transformation|GetActorLocation) (Math|Vector|RotateVector (- _location (Math|Vector|MakeVector _x 0.0 0.0)) _returnvalue_2)) (+ (Transformation|GetActorLocation) (Math|Vector|RotateVector (+ _location (Math|Vector|MakeVector _x 0.0 0.0)) _returnvalue_2)) (Math|Vector|MakeVector 1.0 _y _z) (Math|Rotator|MakeRotator (+ _roll _roll_3) (+ _pitch _pitch_3) (+ _yaw _yaw_3)) (Utilities|Array|MakeArray "ObjectTypeQuery1" "ObjectTypeQuery3" "ObjectTypeQuery6" "ObjectTypeQuery5") false 0 "None" true :!label _label))
      (if _returnvalue_4
        (bind _return_2 (CallFunction|FilterCollisionHit _outhits_2))
        (if _return_2
          (return true)
          (else
            (return false)))
        (else
          (return true))))
    (else
      (goto _label))))

(fn FindCupboard
  (bind _returnvalue (Transformation|GetActorLocation))
  ;[0 0 0] Find Cupboard Actor Using Overlap
  (bind _outhits (Collision|MultiSphereTraceForObjects _returnvalue _returnvalue 5.0 (Utilities|Array|MakeArray "ObjectTypeQuery2") false 0 "None"))
  (for _array_element _outhits
    (bind _asbp_cupboard (Utilities|Casting|CastToBP_Cupboard (.HitActor (Collision|BreakHitResult _array_element))))
    (return _asbp_cupboard))
  (return 0))

(fn IsParentalCupboard
  (bind _returnvalue (Transformation|GetActorLocation))
  (bind _build_data (Variables|Default|GetBuild%20Data))
  (bind _collisiontransform (Utilities|Struct|BreakS_Building _build_data))
  (bind (_location _rotation _scale) (Math|Transform|BreakTransform _collisiontransform))
  (bind _returnvalue_2 (+ _returnvalue _location))
  ;[0 0 0] Find Cupboard Actor Using Overlap
  (bind _outhits (Class|KismetSystemLibrary|BoxTraceMultiforObjects _returnvalue_2 _returnvalue_2 _scale (Math|Rotator|CombineRotators (Transformation|GetActorRotation) _rotation) (Utilities|Array|MakeArray "ObjectTypeQuery2") false 0 "None" true))
  (for _array_element _outhits
    (bind _asbp_cupboard (Utilities|Casting|CastToBP_Cupboard (.HitActor (Collision|BreakHitResult _array_element))))
    (if (Utilities|Array|ContainsItem (Variables|/Game/UltimateSurvivalPack/Blueprints/Buildings/Final/BP_Cupboard.BP_Cupboard_C|GetPrivilege%20Players _asbp_cupboard) (Variables|/Game/UltimateSurvivalPack/Blueprints/Components/BP_PlayerComponent.BP_PlayerComponent_C|GetPlayer%20Unique%20ID (CallFunction|GetPlayerComponent (Variables|Actor|GetInstigator))))
      (if (<= (Math|Vector|Distance(Vector) (Transformation|GetActorLocation) (Transformation|GetActorLocation _asbp_cupboard)) (Variables|/Game/UltimateSurvivalPack/Blueprints/Buildings/Final/BP_Cupboard.BP_Cupboard_C|GetCupboard%20Distance _asbp_cupboard))
        (LocalVariables|SetL%20Cupboard _asbp_cupboard))
      (else
        (return false 0))))
  (return true (LocalVariables|GetL%20Cupboard)))

(fn CanLockLocation
  (params (Hit%20Result :type Hit%20Result%20Structure))
  (return true))

(fn VectorModification
  (params (Vector :type Vector))
  (return (Math|Vector|MakeVector (.x Vector) (.y Vector) (Math|Float|Clamp(Float) (.z Vector) -125.0 125.0))))

(fn FilterCollisionHit
  (params (Filter :type Array%20of%20Hit%20Result%20Structures))
  (for _array_element Filter
    (if (not (Utilities|Array|ContainsItem (Variables|Default|GetCollision%20Class%20Filter) (Utilities|GetClass (.HitActor (Collision|BreakHitResult _array_element)))))
      (return false)))
  (return true))