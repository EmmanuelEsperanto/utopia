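; Interactable, lockpickable treasure chest that ejects one random item stack when opened and can respawn.
; Interaction starts lockpicking or sets Opened, whose RepNotify drives lid, glow, sound and smoke, and reinitializes the lock on respawn.
; After the opening animation, the authority spawns loot by rerolling SpawnerData rows against Chance (higher is rarer), falling back to DT_ItemData without a table.
; Selection highlights the closed chest through custom depth stencil.
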(event Custom|Toggle%20Chest
  (Variables|Default|SetOpened true))

(event Custom|Toggle%20Chest%20Animation%20and%20Spawn
  (params (Toggle :type Boolean))
  (if Toggle
    (Audio|Components|Audio|FadeOut (Variables|Default|GetCUE_TreasureNoise) 2.0 0.0 "Logarithmic" :!class /Script/Engine.AudioComponent)
    (Audio|SpawnSoundatLocation "/Game/UltimateSurvivalPack/Demo/Audio/SFX/CUE_TreasureOpen.CUE_TreasureOpen" (Transformation|GetActorLocation) "0, 0, 0" 0.8 1.0 0.0 "/Game/UltimateSurvivalPack/Blueprints/Attenuation/SA_Footsteps.SA_Footsteps" 0)
    (Components|Activation|SetActive (Variables|Default|GetP_ShineSmoke) false false)
    (bind _alpha (Timeline|Animation PlayFromStart)
      (:Update
        (Transformation|SetRelativeRotation (Variables|Default|GetChestPart) (Math|Rotator|MakeRotator 0.0 (* _alpha -8e+01) 0.0) false false)
        (Rendering|Material|SetScalarParameterValue (Variables|Default|GetTreasure%20Material) "Emissive" (- 1.0 _alpha) :!class /Script/Engine.MaterialInstanceDynamic))
      (:Finished
        (Networking|SwitchHasAuthority
          (:Authority
            (if (Variables|Default|GetOpened)
              (bind _item_to_spawn (CallFunction|GetRandomItemtoSpawn))
              ;[1 1 1] Spawn Item And Add Impulse
              (bind _returnvalue (Game|SpawnActorfromClass "/Game/UltimateSurvivalPack/Blueprints/BP_InventoryItem.BP_InventoryItem_C" (Math|Transform|MakeTransform (Transformation|GetWorldLocation (Variables|Default|GetSpawnLocation)) (Transformation|GetWorldRotation (Variables|Default|GetChestPart))) "AdjustIfPossibleButAlwaysSpawn" 0 _item_to_spawn 0 0))
              (Physics|AddImpulse (Variables|/Game/UltimateSurvivalPack/Blueprints/BP_InventoryItem.BP_InventoryItem_C|GetItem%20Mesh _returnvalue) (+ (* (Transformation|GetActorForwardVector) -2.5e+02) "0, 0,300.000000") "None" true))))))
    (else
      (Audio|Components|Audio|FadeOut (Variables|Default|GetCUE_TreasureNoise) 2.0 1.0 "Logarithmic" :!class /Script/Engine.AudioComponent)
      (Components|Activation|SetActive (Variables|Default|GetP_ShineSmoke) true true)
      (Timeline|Animation ReverseFromEnd))))

(event EventRequestRespawn
  (Variables|Default|SetOpened false))

(event EventToggleSelected
  (params (Toggle :type Boolean))
  (bind _chestpart (Variables|Default|GetChestPart))
  (bind _chestpart_2 (Variables|Default|GetChestPart))
  ;[1 1 1] On Selected
  (if (Variables|Default|GetOpened)
    (Rendering|SetRenderCustomDepth _chestpart false :!label _label)
    (Rendering|SetCustomDepthStencilValue _chestpart 0)
    (elif Toggle
      (Rendering|SetRenderCustomDepth _chestpart_2 true)
      (Rendering|SetCustomDepthStencilValue _chestpart_2 1)
      (else
        (goto _label)))))

(event EventOnInteracted
  (params (Executor :type Controller%20Object%20Reference))
  (bind _bp_lockpickcomponent (Variables|Default|GetBP_LockpickComponent))
  ;[1 1 1] On Interacted
  (if (not (Variables|Default|GetOpened))
    ;;[1 1 1] Lockpick Conditions
    (bind (_return _is_unlocked) (Default|CanLockpick _bp_lockpickcomponent Executor))
    (if _return
      (Default|ToggleLockpicking _bp_lockpickcomponent Executor)
      (elif _is_unlocked
        (CallFunction|ToggleChest)))))

(fn ConstructionScript
  (bind _returnvalue (Rendering|Material|CreateDynamicMaterialInstance "/Game/UltimateSurvivalPack/Demo/Material/M_TreasureChest.M_TreasureChest" "None" "None" :!class /Script/Engine.KismetMaterialLibrary))
  (bind _output_get (Variables|Default|SetTreasure%20Material _returnvalue))
  (Rendering|Material|SetMaterial (Variables|Default|GetChest) 0 _output_get)
  (Rendering|Material|SetMaterial (Variables|Default|GetChestPart) 0 _output_get))

(fn OnRepOpened
  (bind _opened (Variables|Default|GetOpened))
  (CallFunction|ToggleChestAnimationandSpawn _opened)
  (if (not _opened)
    (Default|InitializeLockpickComponent (Variables|Default|GetBP_LockpickComponent))))

(fn GetRandomItemtoSpawn
  (Utilities|IsValid (Variables|Default|GetSpawner%20Data)
    (:Is%20Valid
      (bind _outrownames (DataTable|GetDataTableRowNames (Variables|Default|GetSpawner%20Data)))
      (bind _returnvalue (Utilities|GetDataTableRow (Variables|Default|GetSpawner%20Data) (Utilities|Array|Get(acopy) _outrownames (Math|Random|RandomIntegerinRange 0 (Utilities|Array|LastIndex _outrownames))) :!label _label)
        (:then
          (bind _output_get (LocalVariables|SetL%20Selected%20Item _returnvalue))
          (if (>= (Math|Random|RandomFloatinRange 0.0 1.0) (.Chance (Utilities|Struct|BreakS_ItemSpawner _output_get)))
            (return (Utilities|Struct|MakeS_InventoryItem (.id (LocalVariables|GetL%20Selected%20Item)) (Math|Integer|Clamp(Integer) (Math|Random|RandomIntegerinRange (.minimumspawnamount (LocalVariables|GetL%20Selected%20Item)) (.maximumspawnamount (LocalVariables|GetL%20Selected%20Item))) 1 (.MaximumStack (Utilities|Struct|BreakS_InventoryItemData (.Item%20Data (CallFunction|GetItemDatafromID (.id (LocalVariables|GetL%20Selected%20Item))))))) 0 0 0 1.0 0))
            (else
              (goto _label))))))
    (:Is%20Not%20Valid
      (bind _outrownames_2 (DataTable|GetDataTableRowNames "/Game/UltimateSurvivalPack/Blueprints/Datatable/Inventory/DT_ItemData.DT_ItemData"))
      (LocalVariables|SetL%20Selected%20Item (Utilities|Struct|MakeS_ItemSpawner (Utilities|Array|Get(acopy) _outrownames_2 (Math|Random|RandomIntegerinRange 0 (Utilities|Array|LastIndex _outrownames_2))) 0 0 0.0))
      (return (Utilities|Struct|MakeS_InventoryItem (.id (LocalVariables|GetL%20Selected%20Item)) (Math|Random|RandomIntegerinRange 1 (.MaximumStack (Utilities|Struct|BreakS_InventoryItemData (.Item%20Data (CallFunction|GetItemDatafromID (.id (LocalVariables|GetL%20Selected%20Item))))))) 0 0 0 1.0 0)))))

(fn GetInteractionData
  (if (Variables|Default|GetOpened)
    (return "")
    (elif (Variables|/Game/UltimateSurvivalPack/Blueprints/Components/BP_LockpickComponent.BP_LockpickComponent_C|GetLocked (Variables|Default|GetBP_LockpickComponent))
      (return "Lockpick Treasure Chest")
      (else
        (return "Open Treasure Chest")))))

(fn GetTeamID
  (return 0))

(fn LocalCanOverlap
  (return false))