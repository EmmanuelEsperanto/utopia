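; Curved stairs building part that supplies snap-point data for a building system.
; Per-category getters return hard-coded transforms for floor, ground, roof and wall attachments, while foundation and special getters return no locations.
; A part-type getter reports its enum category, and most transforms carry non-uniform, zeroed-axis scale vectors.
; The event graph and construction script hold no logic, so the asset is purely data.
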(event EventBeginPlay)

(event Collision|EventActorBeginOverlap
  (params (OtherActor :type Actor%20Object%20Reference)))

(event EventTick
  (params (DeltaSeconds :type Float%20%28single-precision%29)))

(fn ConstructionScript)

(fn GetFloorLocations
  (return (Utilities|Array|MakeArray (Math|Transform|MakeTransform "-250.000000, 0,125.000000" "0, 0, 0" "1,0.000000,0.000000") (Math|Transform|MakeTransform "250.000000, 0,250.000000" "0, 0, 0" "1,0.000000,0.000000"))))

(fn GetFoundationLocations
  (return 0))

(fn GetGroundLocations
  (return (Utilities|Array|MakeArray (Math|Transform|MakeTransform "250.000000, 0,250.000000" "0,180.000000, 0" "0.000000,0.000000,1"))))

(fn GetPartType
  (return "NewEnumerator3"))

(fn GetRoofLocations
  (return (Utilities|Array|MakeArray (Math|Transform|MakeTransform "125.000000, 0,250.000000"))))

(fn GetSpecialLocations
  (return 0))

(fn GetWallLocations
  (return (Utilities|Array|MakeArray (Math|Transform|MakeTransform "125.000000, 0,250.000000" "0, 0, 0" "0.000000,1,0.000000"))))