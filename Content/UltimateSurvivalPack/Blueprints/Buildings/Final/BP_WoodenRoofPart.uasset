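; Wooden roof building piece from the survival pack's building system, defined by its part type and the snap points it offers to other pieces.
; Getter functions return hardcoded transforms for floor, roof and wall attachments, while foundation, ground and special getters return no locations.
; The event graph and construction script are empty, so the Blueprint only supplies placement data.
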(event EventBeginPlay)

(event Collision|EventActorBeginOverlap
  (params (OtherActor :type Actor%20Object%20Reference)))

(event EventTick
  (params (DeltaSeconds :type Float%20%28single-precision%29)))

(fn ConstructionScript)

(fn GetFloorLocations
  (return (Utilities|Array|MakeArray (Math|Transform|MakeTransform "-375.000000, 0,250.000000"))))

(fn GetFoundationLocations
  (return 0))

(fn GetGroundLocations
  (return 0))

(fn GetPartType
  (return "NewEnumerator5"))

(fn GetRoofLocations
  (return (Utilities|Array|MakeArray (Math|Transform|MakeTransform "-250.000000, 0,250.000000"))))

(fn GetSpecialLocations
  (return 0))

(fn GetWallLocations
  (return (Utilities|Array|MakeArray (Math|Transform|MakeTransform "0, 0, 0") (Math|Transform|MakeTransform "-250.000000,0.000000,250.000000"))))