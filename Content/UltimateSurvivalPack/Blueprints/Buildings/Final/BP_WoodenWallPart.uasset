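; BP_WoodenWallPart is the wooden wall piece of a modular building system, defining where other parts can attach to it.
; Getter functions report its part type and hard-coded local transforms for each kind of attachable part.
; Walls and roofs stack on top, while flat and angled floors attach at top height on either side.
; Foundation, ground and special getters return nothing, and the event graph and construction script hold no logic.
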(event EventBeginPlay)

(event Collision|EventActorBeginOverlap
  (params (OtherActor :type Actor%20Object%20Reference)))

(event EventTick
  (params (DeltaSeconds :type Float%20%28single-precision%29)))

(fn ConstructionScript)

(fn GetAngledFloorLocations
  (return (Utilities|Array|MakeArray (Math|Transform|MakeTransform "72.500000, 0,250.000000" "0,-30.000000, 0") (Math|Transform|MakeTransform "-72.500000, 0,250.000000" "0,30.000000, 0"))))

(fn GetAngledFoundationLocations
  (return 0))

(fn GetFloorLocations
  (return (Utilities|Array|MakeArray (Math|Transform|MakeTransform "125.000000, 0,250.000000") (Math|Transform|MakeTransform "-125.000000, 0,250.000000"))))

(fn GetFoundationLocations
  (return 0))

(fn GetGroundLocations
  (return 0))

(fn GetPartType
  (return "NewEnumerator1"))

(fn GetRoofLocations
  (return (Utilities|Array|MakeArray (Math|Transform|MakeTransform "0, 0,250.000000" "0, 0, 0" "1,1,1"))))

(fn GetSpecialLocations
  (return 0))

(fn GetWallLocations
  (return (Utilities|Array|MakeArray (Math|Transform|MakeTransform "0, 0,250.000000" "0, 0, 0" "1,1,1"))))