(event Custom|Add%20Building
  (params (Building%20ID :type String))
  (Utilities|Array|AddUnique (Variables|Default|GetPrivilege%20Buildings) Building%20ID)
  (CallFunction|SaveBuildingList))

(event Custom|Remove%20Building
  (params (Building%20ID :type String))
  (Utilities|Array|RemoveItem (Variables|Default|GetPrivilege%20Buildings) Building%20ID)
  (CallFunction|SaveBuildingList))

(event Custom|Set%20Building%20Overlap%20Color
  (params (Overlap :type Boolean))
  (Rendering|Material|SetVectorParameterValue (Variables|Default|GetDynamic%20Zone%20Material) "Color" (select Overlap "(R=0.143218,G=0.500000,B=0.038540,A=1.000000)" "(R=0.500000,G=0.500000,B=0.500000,A=1.000000)") :!class /Script/Engine.MaterialInstanceDynamic))

(event EventOnInteracted
  (params (Executor :type Controller%20Object%20Reference))
  ;[1 1 1] Add To Cupboard
  (bind _asplayer_controller (Utilities|Casting|CastToPlayerController Executor))
  (if (not (Utilities|Array|ContainsItem (Variables|Default|GetPrivilege%20Players) (CallFunction|GetPlayerUniqueID _asplayer_controller)))
    (Utilities|Array|AddUnique (Variables|Default|GetPrivilege%20Players) (CallFunction|GetPlayerUniqueID _asplayer_controller))
    (Networking|FlushNetDormancy)
    (CallFunction|SavePlayerList)
    (Default|CLIENTAddNotification (CallFunction|GetLevelingComponent _asplayer_controller) (Utilities|Struct|MakeS_Notification "Added To Cupboard" "You have been privileged"))))

(event EventToggleSelected
  (params (Toggle :type Boolean))
  (bind _staticmesh (Variables|Default|GetStaticMesh))
  (bind _staticmesh_2 (Variables|Default|GetStaticMesh))
  ;[1 1 1] Select
  (if Toggle
    (Rendering|SetRenderCustomDepth _staticmesh_2 true)
    (Rendering|SetCustomDepthStencilValue _staticmesh_2 1)
    (else
      (Rendering|SetRenderCustomDepth _staticmesh false)
      (Rendering|SetCustomDepthStencilValue _staticmesh 0))))

(event EventBeginPlay
  (Networking|SwitchHasAuthority
    (:Authority
      (Utilities|FlowControl|Delay 0.0) ; Wait for Save Loading
      (if (<= (Utilities|Array|Length (Variables|Default|GetPrivilege%20Buildings)) 0)
        (CallFunction|FindPrivilegeBuilding)))))

(fn ConstructionScript
  ;[1 1 1] Create Dynamic Zone Material
  (bind _returnvalue (Rendering|Material|CreateDynamicMaterialInstance (Variables|Default|GetZone) 0 "/Game/UltimateSurvivalPack/Material/M_BuildZone.M_BuildZone" "None" :!class /Script/Engine.PrimitiveComponent))
  (Variables|Default|SetDynamic%20Zone%20Material _returnvalue))

(fn SavePlayerList
  (bind _assurvival_gamemode (Utilities|Casting|CastToSurvivalGamemode (Game|GetGameMode)))
  (if (.ReturnValue (Default|GetSavedBuildData _assurvival_gamemode (Variables|/Game/UltimateSurvivalPack/Blueprints/Buildings/Parent/BP_BuildingComponent.BP_BuildingComponent_C|GetBuild%20ID (Actor|GetComponentbyClass "/Game/UltimateSurvivalPack/Blueprints/Buildings/Parent/BP_BuildingComponent.BP_BuildingComponent_C"))))
    (for _array_element (Variables|Default|GetPrivilege%20Players)
      (Utilities|Array|Add (LocalVariables|GetL%20Players) (Utilities|Struct|MakeS_InventoryItem (Utilities|String|StringToName _array_element) 0 0 0 0 1.0 0)))
    (bind _structout (Utilities|Struct|SetmembersinS_BuildSave (.Saved%20Data (Default|GetSavedBuildData _assurvival_gamemode (Variables|/Game/UltimateSurvivalPack/Blueprints/Buildings/Parent/BP_BuildingComponent.BP_BuildingComponent_C|GetBuild%20ID (Actor|GetComponentbyClass "/Game/UltimateSurvivalPack/Blueprints/Buildings/Parent/BP_BuildingComponent.BP_BuildingComponent_C")))) (LocalVariables|GetL%20Players)))
    (Default|SaveExistingBuilding _assurvival_gamemode (Variables|/Game/UltimateSurvivalPack/Blueprints/Buildings/Parent/BP_BuildingComponent.BP_BuildingComponent_C|GetBuild%20ID (Actor|GetComponentbyClass "/Game/UltimateSurvivalPack/Blueprints/Buildings/Parent/BP_BuildingComponent.BP_BuildingComponent_C")) _structout)))

(fn FindPrivilegeBuilding
  (bind _returnvalue (Transformation|GetActorLocation))
  (bind _returnvalue_2 (Actor|GetComponentbyClass "/Game/UltimateSurvivalPack/Blueprints/Buildings/Parent/BP_BuildingComponent.BP_BuildingComponent_C"))
  (bind _build_id (Variables|/Game/UltimateSurvivalPack/Blueprints/Buildings/Parent/BP_BuildingComponent.BP_BuildingComponent_C|GetBuild%20ID _returnvalue_2))
  (bind (_outhits _returnvalue_3) (Collision|MultiSphereTraceForObjects _returnvalue _returnvalue (Variables|Default|GetCupboard%20Distance) (Utilities|Array|MakeArray "ObjectTypeQuery1" "ObjectTypeQuery6") false 0 "None"))
  (if _returnvalue_3
    (for _array_element _outhits
      (if (not (Utilities|Array|ContainsItem (LocalVariables|GetL%20Actor%20List) (.HitActor (Collision|BreakHitResult _array_element))))
        (if (<= (Transformation|GetDistanceTo (.HitActor (Collision|BreakHitResult _array_element)) self) (Variables|Default|GetCupboard%20Distance))
          (Utilities|IsValid (Actor|GetComponentbyClass (.HitActor (Collision|BreakHitResult _array_element)) "/Game/UltimateSurvivalPack/Blueprints/Buildings/Parent/BP_BuildingComponent.BP_BuildingComponent_C")
            (:Is%20Valid
              (Utilities|Array|AddUnique (Variables|Default|GetPrivilege%20Buildings) (Variables|/Game/UltimateSurvivalPack/Blueprints/Buildings/Parent/BP_BuildingComponent.BP_BuildingComponent_C|GetBuild%20ID (Actor|GetComponentbyClass (.HitActor (Collision|BreakHitResult _array_element)) "/Game/UltimateSurvivalPack/Blueprints/Buildings/Parent/BP_BuildingComponent.BP_BuildingComponent_C")))
              ;[1 1 1] Set Cupboard ID with Save
              (Default|SetCupboard (Actor|GetComponentbyClass (.HitActor (Collision|BreakHitResult _array_element)) "/Game/UltimateSurvivalPack/Blueprints/Buildings/Parent/BP_BuildingComponent.BP_BuildingComponent_C") (Variables|/Game/UltimateSurvivalPack/Blueprints/Buildings/Parent/BP_BuildingComponent.BP_BuildingComponent_C|GetBuild%20ID (Actor|GetComponentbyClass "/Game/UltimateSurvivalPack/Blueprints/Buildings/Parent/BP_BuildingComponent.BP_BuildingComponent_C"))))))))
    ;[1 1 1] Save Building
    (bind _assurvival_gamemode (Utilities|Casting|CastToSurvivalGamemode (Game|GetGameMode)))
    (if (.ReturnValue (Default|GetSavedBuildData _assurvival_gamemode _build_id))
      (bind _structout (Utilities|Struct|SetmembersinS_BuildSave (.Saved%20Data (Default|GetSavedBuildData _assurvival_gamemode _build_id)) (Variables|Default|GetPrivilege%20Buildings)))
      (Default|SaveExistingBuilding _assurvival_gamemode _build_id _structout))))

(fn SaveBuildingList
  (bind _returnvalue (Actor|GetComponentbyClass "/Game/UltimateSurvivalPack/Blueprints/Buildings/Parent/BP_BuildingComponent.BP_BuildingComponent_C"))
  (bind _build_id (Variables|/Game/UltimateSurvivalPack/Blueprints/Buildings/Parent/BP_BuildingComponent.BP_BuildingComponent_C|GetBuild%20ID _returnvalue))
  (bind _assurvival_gamemode (Utilities|Casting|CastToSurvivalGamemode (Game|GetGameMode)))
  (if (.ReturnValue (Default|GetSavedBuildData _assurvival_gamemode _build_id))
    (bind _structout (Utilities|Struct|SetmembersinS_BuildSave (.Saved%20Data (Default|GetSavedBuildData _assurvival_gamemode _build_id)) (Variables|Default|GetPrivilege%20Buildings)))
    (Default|SaveExistingBuilding _assurvival_gamemode _build_id _structout)))

(fn GetInteractionData
  (return "Add to Cupboard"))

(fn GetTeamID
  (return 0))

(fn LocalCanOverlap
  (return false))