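; BP_Campfire is a campfire building that warms the local player and shows fire effects when its refinery action toggles.
; A looping timeline flickers the point light's intensity, while the toggle switches the Niagara fire, looping sound and light visibility.
; Local overlap, range-checked at 600 units by squared distance, sets the player component's AdditionalTemperature on entry and subtracts it on exit.
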(event EventBeginPlay
  (|CallParentFunction)
  (bind _alpha (Timeline|Light%20Effect Play)
    (:Update
      (Rendering|Components|Light|SetIntensity (Variables|Default|GetPointLight) (* _alpha 5e+03)))
    (:Finished
      (Timeline|Light%20Effect PlayFromStart))))

(event EventLocalOverlap
  (params (Overlap :type Boolean))
  (bind _returnvalue (Game|GetPlayerController 0))
  (bind _returnvalue_2 (CallFunction|GetInventoryComponent _returnvalue))
  (bind _human_player_character (Variables|/Game/UltimateSurvivalPack/Blueprints/Components/BP_PlayerInventoryComponent.BP_PlayerInventoryComponent_C|GetHuman%20Player%20Character _returnvalue_2))
  (bind _returnvalue_3 (CallFunction|GetPlayerComponent _human_player_character))
  (if Overlap
    (Variables|/Game/UltimateSurvivalPack/Blueprints/Components/BP_PlayerComponent.BP_PlayerComponent_C|SetAdditional%20Temperature _returnvalue_3 (Variables|Default|GetAdditional%20Temperature))
    (else
      (Variables|/Game/UltimateSurvivalPack/Blueprints/Components/BP_PlayerComponent.BP_PlayerComponent_C|SetAdditional%20Temperature _returnvalue_3 (- (Variables|/Game/UltimateSurvivalPack/Blueprints/Components/BP_PlayerComponent.BP_PlayerComponent_C|GetAdditional%20Temperature _returnvalue_3) (Variables|Default|GetAdditional%20Temperature))))))

(event EventToggleRafineryAction
  (params (Toggle :type Boolean))
  (Components|Activation|SetActive (Variables|Default|GetNiagara) Toggle false)
  (Rendering|SetVisibility (Variables|Default|GetPointLight) Toggle false))

(fn ConstructionScript)

(fn LocalCanOverlap
  (return (< (Transformation|GetSquaredDistanceTo (Pawn|GetControlledPawn (Game|GetPlayerController 0))) 3.6e+05)))