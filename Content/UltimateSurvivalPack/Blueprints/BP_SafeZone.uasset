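; BP_SafeZone is a safe zone actor that flags the local player's inventory component while they are inside its area.
; One second after BeginPlay it registers itself as a custom marker with the player's mission component.
; LocalCanOverlap tests the player pawn's distance against the Sphere radius, and the LocalOverlap event passes enter or exit state to SetSafezone.
; Interaction data and team ID return empty defaults.
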(event EventBeginPlay
  (Utilities|FlowControl|Delay 1.0)
  (Default|AddCustomMarker (CallFunction|GetMissionComponent (Game|GetPlayerController 0)) (Variables|Default|GetMarker) self))

(event EventLocalOverlap
  (params (Overlap :type Boolean))
  ;[1 1 1] Enter Area Event
  (Default|SetSafezone (CallFunction|GetInventoryComponent (Game|GetPlayerController 0)) Overlap))

(fn ConstructionScript)

(fn GetInteractionData
  (return ""))

(fn GetTeamID
  (return 0))

(fn LocalCanOverlap
  (return (< (Transformation|GetDistanceTo (Game|Player|GetPlayerPawn 0)) (Components|Sphere|GetScaledSphereRadius (Variables|Default|GetSphere)))))