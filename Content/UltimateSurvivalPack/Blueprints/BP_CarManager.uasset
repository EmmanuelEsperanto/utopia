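; BP_CarManager is an interactable actor owned by a BP_Garage that opens the "Customize Car" screen.
; On interaction it takes the garage's VehicleReference and, if valid, calls CLIENTOpenVehicleCustomization on the executor's inventory component.
; Selection toggles a custom depth stencil highlight on its Cube.
; It reports team 0 and disallows local overlap.
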(event EventToggleSelected
  (params (Toggle :type Boolean))
  (bind _cube (Variables|Default|GetCube))
  (bind _cube_2 (Variables|Default|GetCube))
  ;[1 1 1] On Selected
  (if Toggle
    (Rendering|SetRenderCustomDepth _cube_2 true)
    (Rendering|SetCustomDepthStencilValue _cube_2 1)
    (else
      (Rendering|SetRenderCustomDepth _cube false)
      (Rendering|SetCustomDepthStencilValue _cube 0))))

(event EventOnInteracted
  (params (Executor :type Controller%20Object%20Reference) (HitComponent :type Scene%20Component%20Object%20Reference))
  (bind _asbp_garage (Utilities|Casting|CastToBP_Garage (Components|GetOwner)))
  (bind _vehicle_reference (Variables|/Game/UltimateSurvivalPack/Blueprints/BP_Garage.BP_Garage_C|GetVehicle%20Reference _asbp_garage)
    (:then
      (Default|CLIENTOpenVehicleCustomization (CallFunction|GetInventoryComponent Executor) _vehicle_reference))
    (:else)))

(fn ConstructionScript)

(fn GetInteractionData
  (return "Customize Car"))

(fn GetTeamID
  (return 0))

(fn LocalCanOverlap
  (return false))