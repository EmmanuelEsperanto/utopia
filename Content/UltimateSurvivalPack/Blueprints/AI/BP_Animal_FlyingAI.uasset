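; Flying animal AI pawn for birds that roam around their spawner.
; A looping timer, with its interval randomized once at start, picks random goal points in a box around the spawner.
; While alive it constantly moves forward in flying mode, with the server smoothly steering its rotation toward the goal.
; Construction picks one of three bird materials, and multicast death enables mesh physics and sets the material's Dead parameter.
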(event EventBeginPlay
  (bind _goal_update_time (Variables|Default|GetGoal%20Update%20Time))
  (|CallParentFunction)
  (Pawn|Components|CharacterMovement|SetMovementMode (Variables|Character|GetCharacterMovement) "MOVE_Flying" 0)
  (Utilities|FlowControl|Delay 0.5)
  (Utilities|Time|SetTimerbyFunctionName 0 "Find New Goal Location" (Math|Random|RandomFloatinRange (* _goal_update_time 0.5) (* _goal_update_time 1.5)) true 5.0)
  (CallFunction|FindNewGoalLocation))

(event EventTick
  (params (DeltaSeconds :type Float%20%28single-precision%29))
  (|CallParentFunction DeltaSeconds)
  (if (Variables|/Game/UltimateSurvivalPack/Blueprints/Components/BP_AI_DataComponent.BP_AI_DataComponent_C|GetIs%20Alive (Variables|Default|GetC_AI_DataComponent))
    (Pawn|Input|AddMovementInput (Transformation|GetActorForwardVector) 1.0 false)
    (Networking|SwitchHasAuthority
      (:Authority
        (Transformation|SetActorRotation (Math|Interpolation|RInterpTo (Transformation|GetActorRotation) (Math|Rotator|FindLookatRotation (Transformation|GetActorLocation) (Variables|Default|GetGoal%20Location)) (Utilities|Time|GetWorldDeltaSeconds) (Variables|Default|GetRotation%20Speed)))))))

(event EventMULTICASTonDead
  (|CallParentFunction)
  (Physics|SetSimulatePhysics (Variables|Character|GetMesh) true)
  (Rendering|Material|SetScalarParameterValue (Variables|Default|GetDynamic%20Material) "Dead" 1.0 :!class /Script/Engine.MaterialInstanceDynamic))

(fn ConstructionScript
  (|CallParentFunction)
  (Pawn|Components|CharacterMovement|SetMovementMode (Variables|Character|GetCharacterMovement) "MOVE_Flying" 0)
  (bind _returnvalue (Rendering|Material|CreateDynamicMaterialInstance (Utilities|Select :Index (Math|Random|RandomIntegerinRange 0 2) :Option%200 "/Game/UltimateSurvivalPack/Demo/Animals/Material/M_Animals_Bird_01.M_Animals_Bird_01" :Option%201 "/Game/UltimateSurvivalPack/Demo/Animals/Material/M_Animals_Bird_02.M_Animals_Bird_02" :Option%202 "/Game/UltimateSurvivalPack/Demo/Animals/Material/M_Animals_Bird_03.M_Animals_Bird_03") "None" "None" :!class /Script/Engine.KismetMaterialLibrary))
  (Variables|Default|SetDynamic%20Material _returnvalue)
  (Rendering|Material|SetMaterial (Variables|Character|GetMesh) 0 _returnvalue))

(fn FindNewGoalLocation
  (bind _flying_distance (Variables|Default|GetFlying%20Distance))
  (Variables|Default|SetGoal%20Location (Math|Random|RandomPointinBoundingBox (Transformation|GetActorLocation (Variables|Default|GetSpawner%20Reference)) (Math|Vector|MakeVector _flying_distance _flying_distance 1e+03))))