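; Target component that links an actor to the player's mission component as a possible objective target, handling its markers and progress reports.
; While the locally controlled pawn overlaps, a looping timer adds markers if the target is in the current objectives and removes stale ones.
; Ending overlap destroys the markers and stops the timer.
; Interaction reports progress to the interacting player's mission component, including joined players.
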(event Custom|Overlap%20Refresh
  (bind _returnvalue (Game|GetPlayerController 0))
  (bind _target_information (Variables|Default|GetTarget%20Information))
  (bind _missioncomponent (CallFunction|GetMissionComponent _returnvalue))
  (bind (_objective_index _objective_target _successful) (Default|FindTargetinCurrentObjectives _missioncomponent _target_information))
  ;[1 1 1] Overlapping Events (Checking every 0.25 if marker should or shouldn't create)
  (if (> (Utilities|Array|Length (Variables|Default|GetMarker%20Reference)) 0)
    (if (UserInterface|Viewport|IsinViewport (Utilities|Array|Get(acopy) (Variables|Default|GetMarker%20Reference)))
      ;;[1 0.1 0.1] Remove Marker If Is Valid but not needed
      (if (not _successful)
        (for _array_element (Variables|Default|GetMarker%20Reference) :!label _label
          (Default|DestroyMarkerReference (CallFunction|GetMissionComponent (Game|GetPlayerController 0)) _array_element))
        (Utilities|Array|Clear (Variables|Default|GetMarker%20Reference)))
      (else
        (goto _label)))
    (elif (Variables|/Game/UltimateSurvivalPack/Blueprints/Components/BP_MissionComponent.BP_MissionComponent_C|GetIs%20In%20Mission%20? _missioncomponent)
      (if _successful
        (bind _marker_reference (Default|AddMarker _missioncomponent _objective_index _objective_target (Variables|Default|GetTarget%20Information)))
        (bind _output_get (Variables|Default|SetMarker%20Reference _marker_reference))
        (for _array_element_2 _output_get
          (Utilities|IsValid _array_element_2
            (:Is%20Valid
              (Default|PlayHideAnimation _array_element_2 "Reverse" false))))))))

(event Custom|Overlap
  (params (Other%20Actor :type Actor%20Object%20Reference) (Overlap? :type Boolean))
  ;[1 1 1] Overlap Event
  (bind _aspawn (Utilities|Casting|CastToPawn Other%20Actor))
  (if (Pawn|IsLocallyControlled _aspawn)
    (Utilities|IsValid (CallFunction|GetMissionComponent (Pawn|GetController _aspawn))
      (:Is%20Valid
        (if Overlap?
          (CallFunction|OnOverlap)
          (else
            (CallFunction|OnUnoverlap)))))))

(event Custom|Interacted
  (params (Player :type Controller%20Object%20Reference))
  ;[1 1 1] Reveive Progress On Interacted/Killed etc.
  (Utilities|Casting|CastToPlayerController Player)
  (Default|ReceiveProgress (CallFunction|GetMissionComponent Player) (Variables|Default|GetTarget%20Information) (Utilities|Struct|BreakS_TargetInformation (Variables|Default|GetTarget%20Information)) true))

(event Custom|On%20Unoverlap
  ;[1 0.1 0.1] On Unoverlap
  ;[1 1 1] Unoverlap Events
  (if (> (Utilities|Array|Length (Variables|Default|GetMarker%20Reference)) 0)
    (for _array_element (Variables|Default|GetMarker%20Reference)
      (Default|DestroyMarkerReference (CallFunction|GetMissionComponent (Game|GetPlayerController 0)) _array_element))
    (Utilities|Array|Clear (Variables|Default|GetMarker%20Reference)))
  (Utilities|Time|ClearandInvalidateTimerbyHandle (Variables|Default|GetTimer%20Event)))

(event Custom|On%20Overlap
  ;[0.1658 1 0.1] On Overlap
  ;[1 1 1] Overlapping Events (Checking every 0.25 if marker should or shouldn't create)
  (if (not (Utilities|Time|IsValidTimerHandle (Variables|Default|GetTimer%20Event)))
    (bind _returnvalue (Utilities|Time|SetTimerbyEvent (delegate Custom|Overlap%20Refresh) 0.25 true))
    (Variables|Default|SetTimer%20Event _returnvalue)
    (CallFunction|OverlapRefresh)))