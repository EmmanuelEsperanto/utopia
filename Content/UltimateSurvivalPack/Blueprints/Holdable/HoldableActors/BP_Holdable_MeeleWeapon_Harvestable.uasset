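; Melee weapon holdable variant for harvesting, adding a server-side mining swing against actors tagged "Mineable".
; CanMine requires durability and a short sphere trace hit ahead of the instigator.
; The server event then multicasts the mining montage, applies delayed damage and uses a DoOnce cooldown.
; PrimaryAction only calls the parent; the branch that would trigger mining from it is disconnected.
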(event Custom|SERVER%20Play%20Montage
  (bind _return (CallFunction|CanMine))
  (if _return
    (Utilities|FlowControl|DoOnce false :!label _label
      (:Completed
        (CallFunction|MULTICASTPlayMontage)
        (Utilities|FlowControl|Sequence
          (:then_0
            (Utilities|FlowControl|Delay 3.0)
            (goto _label Reset))
          (:then_1
            (Utilities|FlowControl|Delay 1.4)
            (CallFunction|ApplyDamage)))))))

(event Custom|MULTICAST%20Play%20Montage
  (bind _ascharacter (Utilities|Casting|CastToCharacter (Game|GetInstigator)))
  (Animation|PlayAnimMontage _ascharacter "/Game/UltimateSurvivalPack/Demo/Character/Animations/Human/Montage/AM_Mining.AM_Mining" 1.0 "None"))

(event EventPrimaryAction
  (params (Pressed :type Boolean))
  (|CallParentFunction Pressed))

(fn ConstructionScript
  (|CallParentFunction))

(fn CanMine
  (bind _returnvalue (Game|GetInstigator))
  (bind _returnvalue_2 (Transformation|GetActorLocation _returnvalue))
  ;[1 1 1] Has Desired Durability
  (if (Default|HasDurability (CallFunction|GetInventoryComponent (Components|GetOwner)) (.cachedindex (Variables|Default|GetItem%20Data)))
    (bind _outhits (Collision|MultiSphereTraceByChannel _returnvalue_2 (+ _returnvalue_2 (* (Transformation|GetActorForwardVector _returnvalue) 5e+01)) 55.0 "TraceTypeQuery1" false (Utilities|Array|MakeArray (Game|GetInstigator)) "None"))
    (bind _array_element (Utilities|Array|ForEachLoopwithBreak _outhits)
      (:LoopBody
        (if (Utilities|Array|ContainsItem (Variables|/Script/Engine.Actor|GetTags (.HitActor (Collision|BreakHitResult _array_element))) "Mineable")
          (return true)))
      (:Completed
        (return false)))
    (else
      (return false))))