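; Holdable fishing rod that casts a bobber and reels it in to catch random items.
; Primary action, gated by durability and a DoOnce, either spawns an arcing throwable or reels in the existing one; AttachRope links the cable to it.
; Reeling in during catch mode rolls CatchItems by chance-based retry, adding loot to inventory or spawning it in the world.
; Each reel-in costs durability and multicasts the cable detach.
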(event Custom|Spawn%20Projectile
  (params (Throw%20Velocity :type Vector))
  (bind _instigator (Variables|Default|GetInstigator))
  (bind _returnvalue (Game|SpawnActorfromClass "/Game/UltimateSurvivalPack/Blueprints/Holdable/ThrowableActors/BP_Throwable_Fishing.BP_Throwable_Fishing_C" (Math|Transform|MakeTransform (Transformation|GetActorLocation _instigator) "0, 0, 0" "1.000000,1.000000,1.000000") "Undefined" (Components|GetOwner) self Throw%20Velocity _instigator))
  (Variables|Default|SetFishing%20Ball%20Reference _returnvalue))

(event Custom|Emerge%20Rod
  (if (Variables|/Game/UltimateSurvivalPack/Blueprints/Holdable/ThrowableActors/BP_Throwable_Fishing.BP_Throwable_Fishing_C|GetCatch%20Mode (Variables|Default|GetFishing%20Ball%20Reference))
    (bind (_item_id _amount) (CallFunction|GenerateRandomItem))
    (bind _success (Default|AddItem (CallFunction|GetInventoryComponent (Components|GetOwner)) (Utilities|Struct|MakeS_InventoryItem _item_id _amount 0 0 0 1.0 0)))
    (if _success
      _
      (else
        (Game|SpawnActorfromClass "/Game/UltimateSurvivalPack/Blueprints/BP_InventoryItem.BP_InventoryItem_C" (Transformation|GetActorTransform) "Undefined" 0 (Utilities|Struct|MakeS_InventoryItem _item_id _amount 0 0 0 1.0 0) 0 0))))
  (Actor|DestroyActor (Variables|Default|GetFishing%20Ball%20Reference))
  (Default|DeceraseDurability (CallFunction|GetInventoryComponent (Components|GetOwner)) (.cachedindex (Variables|Default|GetItem%20Data)) 0.02)
  (CallFunction|MULTICASTEmergeRod))

(event Custom|Reset%20Action
  (bind _instigator (Variables|Default|GetInstigator))
  (bind _returnvalue (Transformation|GetActorForwardVector _instigator))
  (bind _returnvalue_2 (* _returnvalue 7e+02))
  (Utilities|FlowControl|DoOnce false) ; enters at Reset
)

(event Custom|MULTICAST%20Emerge%20Rod
  (CallFunction|ResetAction)
  (Variables|/Script/CableComponent.CableComponent|SetbAttachEnd (Variables|Default|GetCable) false))

(event Custom|Attach%20Rope
  (params (Fishing%20Ball%20Reference :type BP%20Throwable%20Fishing%20Object%20Reference))
  (bind _cable (Variables|Default|GetCable))
  (Variables|Default|SetFishing%20Ball%20Reference Fishing%20Ball%20Reference)
  (Variables|/Script/CableComponent.CableComponent|SetbAttachEnd _cable true)
  (Class|CableComponent|SetAttachEndto _cable Fishing%20Ball%20Reference "None" "None")
  (CallFunction|ResetAction)
  (Audio|SpawnSoundatLocation "/Game/UltimateSurvivalPack/Demo/Audio/SFX/CUE_PunchSwing.CUE_PunchSwing" (Transformation|GetActorLocation) "0, 0, 0" 1.0 1.0 0.0 "/Game/UltimateSurvivalPack/Blueprints/Attenuation/SA_Footsteps.SA_Footsteps" 0)
  (Development|SetHiddeninGame (Variables|Default|GetCable) false false))

(event Collision|EventActorBeginOverlap
  (params (OtherActor :type Actor%20Object%20Reference)))

(event EventTick
  (params (DeltaSeconds :type Float%20%28single-precision%29)))

(event EventPrimaryAction
  (params (Pressed :type Boolean))
  (bind _instigator (Variables|Default|GetInstigator))
  (bind _returnvalue (Transformation|GetActorForwardVector _instigator))
  (bind _returnvalue_2 (* _returnvalue 7e+02))
  (if Pressed
    (if (Default|HasDurability (CallFunction|GetInventoryComponent (Components|GetOwner)) (.cachedindex (Variables|Default|GetItem%20Data)))
      (Utilities|FlowControl|DoOnce false
        (:Completed
          (Variables|Default|GetFishing%20Ball%20Reference
            (:then
              (CallFunction|EmergeRod))
            (:else
              (CallFunction|SpawnProjectile (Math|Vector|MakeVector (.x _returnvalue_2) (.y _returnvalue_2) 7e+02)))))))))

(event EventDestroyed
  (|CallParentFunction)
  (bind _fishing_ball_reference (Variables|Default|GetFishing%20Ball%20Reference)
    (:then
      (Actor|DestroyActor _fishing_ball_reference))
    (:else)))

(event EventBeginPlay
  (|CallParentFunction)
  (Utilities|FlowControl|Delay 1.0)
  (Development|SetHiddeninGame (Variables|Default|GetCable) false false))

(fn ConstructionScript
  (|CallParentFunction))

(fn GenerateRandomItem
  (bind _catch_items (Variables|Default|GetCatch%20Items))
  (bind _output_get (LocalVariables|SetL%20Item (Utilities|Array|Get(acopy) _catch_items (Math|Random|RandomIntegerinRange 0 (Utilities|Array|LastIndex _catch_items))) :!label _label))
  (if (>= (.ChanceOfSpawning (Utilities|Struct|BreakS_DropItem _output_get)) (Math|Random|RandomFloatinRange 0.0 1.0))
    (return (.ItemID (Utilities|Struct|BreakS_DropItem _output_get)) (Math|Random|RandomIntegerinRange (.MinimumAmount (Utilities|Struct|BreakS_DropItem _output_get)) (.MaximumAmount (Utilities|Struct|BreakS_DropItem _output_get))))
    (else
      (goto _label))))