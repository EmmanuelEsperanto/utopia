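; Holdable tire repair tool that lets a player fix punctured buggy tires using spare tires from the inventory.
; On the owning client, a per-tick camera trace asks vehicles through BPI_VehicleSystem for the hovered tire index and toggles a wrench widget.
; Primary action sends actor and index to a server event, which checks the puncture, consumes a Tire item and calls SERVERRepairTire, or notifies when none is carried.
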(event Custom|SERVER%20Repair%20Tire
  (params (Hit%20Actor :type Actor%20Object%20Reference) (Tire%20Index :type Byte))
  (bind _returnvalue (Components|GetOwner))
  (bind _returnvalue_2 (Utilities|Name|MakeLiteralName "Tire"))
  (bind _returnvalue_3 (CallFunction|GetInventoryComponent _returnvalue))
  (bind _array_index (Default|FindItembyID _returnvalue_3 _returnvalue_2))
  (bind _asbp_buggy (Utilities|Casting|CastToBP_Buggy Hit%20Actor))
  (if (.Success (Default|GetTirebyID _asbp_buggy (Math|Conversions|ToInteger(Byte) Tire%20Index)))
    (if (Utilities|Struct|BreakSTR_WheelStatus (.TireRef (Default|GetTirebyID _asbp_buggy (Math|Conversions|ToInteger(Byte) Tire%20Index))))
      (if (> _array_index -1)
        (Default|RemoveItem _returnvalue_3 _array_index 1 _returnvalue_3)
        (CallFunction|SERVERRepairTire Hit%20Actor Tire%20Index)
        (else
          (Default|CLIENTAddNotification (CallFunction|GetMissionComponent _returnvalue) (Utilities|Struct|MakeS_Notification "Tire Repair" "You do not have any spare tires in your Inventory")))))))

(event EventBeginPlay
  (|CallParentFunction)
  (if (CallFunction|IsOwnerLocal)
    (bind _returnvalue (UserInterface|CreateWidget "/Game/UltimateSurvivalPack/Widget/W_CarWrench.W_CarWrench_C"))
    (Variables|Default|SetCar%20Wrench%20Widget _returnvalue)
    (UserInterface|Viewport|AddtoViewport _returnvalue 0)))

(event EventDestroyed
  (|CallParentFunction)
  (if (CallFunction|IsOwnerLocal)
    (bind _car_wrench_widget (Variables|Default|GetCar%20Wrench%20Widget)
      (:then
        (Widget|RemovefromParent _car_wrench_widget))
      (:else))))

(event EventTick
  (params (DeltaSeconds :type Float%20%28single-precision%29))
  (bind _returnvalue (Game|GetPlayerController 0))
  (bind _returnvalue_2 (Game|GetPlayerCameraManager 0))
  (bind _returnvalue_3 (CallFunction|GetInventoryComponent _returnvalue))
  (bind _returnvalue_4 (Camera|GetCameraLocation _returnvalue_2))
  (|CallParentFunction DeltaSeconds)
  (if (CallFunction|IsOwnerLocal)
    (bind (_outhit _returnvalue_5) (Collision|LineTraceByChannel _returnvalue_4 (+ _returnvalue_4 (* (Math|Vector|GetForwardVector (Camera|GetCameraRotation _returnvalue_2)) (Variables|/Game/UltimateSurvivalPack/Blueprints/Components/BP_PlayerInventoryComponent.BP_PlayerInventoryComponent_C|GetInteraction%20Distance _returnvalue_3))) "TraceTypeQuery1" false (Utilities|Array|MakeArray (Variables|/Game/UltimateSurvivalPack/Blueprints/Components/BP_PlayerInventoryComponent.BP_PlayerInventoryComponent_C|GetHuman%20Player%20Character _returnvalue_3)) "None"))
    (if _returnvalue_5
      (Variables|Default|SetHit%20Actor (.HitActor (Collision|BreakHitResult _outhit)))
      (if (and (Utilities|ClassIsChildOf (Utilities|GetClass (.HitActor (Collision|BreakHitResult _outhit))) 0) (Utilities|DoesObjectImplementInterface (.HitActor (Collision|BreakHitResult _outhit)) "/Game/UltimateSurvivalPack/Blueprints/Interface/BPI_VehicleSystem.BPI_VehicleSystem_C"))
        (bind _punctured_tire_index (Class|BPIVehicleSystem|BPITireSystemHoveredonTire(Message) (.HitActor (Collision|BreakHitResult _outhit)) (.HitComponent (Collision|BreakHitResult _outhit))))
        (bind _output_get (Variables|Default|SetPunctured%20Tire%20Index _punctured_tire_index))
        (Default|Toggle (Variables|Default|GetCar%20Wrench%20Widget) (!= _output_get 255))
        (else
          (Default|Toggle (Variables|Default|GetCar%20Wrench%20Widget) false :!label _label)))
      (else
        (Variables|Default|SetHit%20Actor 0)
        (goto _label)))))

(event EventPrimaryAction
  (params (Pressed :type Boolean))
  (if Pressed
    (if (< (Variables|Default|GetPunctured%20Tire%20Index) 4)
      (bind _hit_actor (Variables|Default|GetHit%20Actor)
        (:then
          (CallFunction|SERVERRepairTire _hit_actor (Variables|Default|GetPunctured%20Tire%20Index)))
        (:else)))))

(fn ConstructionScript
  (|CallParentFunction))