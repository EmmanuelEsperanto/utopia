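; Shotgun subclass of the holdable range weapon that fires multiple pellets per shot and disables fire-mode switching.
; Each pellet sphere-traces from the camera toward a random point in a spread box, then feeds hit filtering, bullet events and recoil; any pawn hit flashes the crosshair once.
; Custom effects draw tracers and impacts per pellet, using a shell counter to play animation, sound and muzzle flash once per shot.
; Damage scales down with distance.
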(event EventChangeFiremode
  ;[1 1 1] Clear FireMode
)

(event EventDoShotAction
  (bind _returnvalue (Game|GetPlayerCameraManager 0))
  (bind _returnvalue_2 (Camera|GetCameraLocation _returnvalue))
  ;[1 1 1] Shot Action
  (if (> (Variables|Default|GetCurrent%20Ammo) 0)
    (for _index (range 1 (Variables|Configuration|Shooting|GetShell%20Amount))
      ;;[1 0.4812 0.3102] Do Hit Trace
      (bind (_outhits _returnvalue_3) (Collision|MultiSphereTraceByChannel _returnvalue_2 (Math|Random|RandomPointinBoundingBox (+ (* (Math|Vector|GetForwardVector (Variables|/Script/Engine.Actor|GetRootComponent _returnvalue)) 5e+04) _returnvalue_2) (Math|Conversions|ToVector(Float) (* (Variables|Configuration|Shooting|GetSpread) 5e+02))) 3.0 "TraceTypeQuery3" true (Utilities|Array|MakeArray (Variables|Default|GetInstigator)) "None"))
      ;;[1 1 1] Hit Filter
      (bind (_surface_hit _water_hit_location) (CallFunction|HitDetection _outhits "0, 0, 0"))
      ;;[1 1 1] Call On Bullet Shot
      (CallFunction|OnBulletShot _returnvalue_3 _surface_hit _water_hit_location)
      (CallFunction|ApplyLocalRecoil)
      (if _returnvalue_3
        (Utilities|Array|Add (Variables|Default|GetHits) _surface_hit)))
    ;;[1 1 1] Decrease Ammo
    (CallFunction|DecreaseAmmo)
    ;;[1 1 1] Play hit animation widget
    (bind _array_element (Utilities|Array|ForEachLoopwithBreak (Variables|Default|GetHits) :!label _label)
      (:LoopBody
        (Utilities|Casting|CastToPawn (.HitActor (Collision|BreakHitResult _array_element))
          (:then
            (Default|OnHit (Variables|/Game/UltimateSurvivalPack/Widget/W_HUD.W_HUD_C|GetW_Crosshair (Variables|/Game/UltimateSurvivalPack/Blueprints/Components/BP_MissionComponent.BP_MissionComponent_C|GetHUD (CallFunction|GetMissionComponent (Game|GetPlayerController 0)))) :!label _label_2)
            (goto _label Break))
          (:CastFailed
            (Utilities|IsValid (.HitComponent (Collision|BreakHitResult _array_element))
              (:Is%20Valid
                (if (Utilities|Enum|Equal(Enum) (Collision|GetCollisionObjectType (.HitComponent (Collision|BreakHitResult _array_element))) "ECC_Pawn")
                  (goto _label_2)))))))
      (:Completed
        (Utilities|Array|Clear (Variables|Default|GetHits))))
    (else
      ;;[1 1 1] Do Custom Effect
      (CallFunction|DoCustomShotEffects false (Collision|MakeHitResult false false 0.0 0.0 "0, 0, 0" "0, 0, 0" "0,0,1" "0,0,1" 0 0) true "0, 0, 0"))))

(fn ConstructionScript
  (|CallParentFunction))

(fn DoCustomShotEffects
  (params (Bullet%20Hit :type Boolean) (Hit%20 :type Hit%20Result%20Structure) (No%20Ammo :type Boolean) (Water%20Hit :type Vector :default "0, 0, 0"))
  (bind (_bblockinghit _binitialoverlap _time _distance _location _impactpoint _normal _impactnormal _physmat _hitactor _hitcomponent _hitbonename _hititem _elementindex _faceindex _tracestart _traceend) (Collision|BreakHitResult Hit%20))
  (bind (_bblockinghit_2 _binitialoverlap_2 _time_2 _distance_2 _location_2 _impactpoint_2 _normal_2 _impactnormal_2 _physmat_2 _hitactor_2 _hitcomponent_2) (Collision|BreakHitResult Hit%20))
  ;[1 0.08333 0.08333] Customize Certain Effect only for Certain weapons
  ;;[1 1 1] Has Enough Ammo?
  (if (not No%20Ammo)
    (LocalVariables|SetPlay%20Effects%20L (== (Variables|Non-Edit|GetShell%20Index) 0))
    (if (>= (Variables|Non-Edit|GetShell%20Index) (- (Variables|Configuration|Shooting|GetShell%20Amount) 1))
      (Variables|Non-Edit|SetShell%20Index 0)
      (else
        (Math|Integer|IncrementInt (Variables|Non-Edit|GetShell%20Index)
          (:%20%20
            _))))
    (if (not (Networking|IsDedicatedServer))
      ;;[1 1 1] Spawn Bullet Trace Effect
      (bind _returnvalue (Niagara|SpawnSystematLocation "/Game/UltimateSurvivalPack/Demo/Particles/Niagara/NS_BulletTrace.NS_BulletTrace" (Transformation|GetWorldLocation (Variables|Default|GetTrigger)) "0, 0, 0" "1.000000,1.000000,1.000000" true false))
      (Effects|Components|ParticleSystem|SetVectorParameter _returnvalue "End Location" (select Bullet%20Hit _impactpoint _traceend))
      (Components|Activation|Activate _returnvalue true)
      (if (LocalVariables|GetPlay%20Effects%20L)
        (if (Variables|Default|GetIs%20Aiming)
          (if (CallFunction|IsFirstPerson)
            _
            (else
              ;;[1 1 1] Play Character Fire Animation
              (bind _asthird_person_character (Utilities|Casting|CastToThirdPersonCharacter (Game|GetInstigator) :!label _label))
              (Utilities|IsValid _asthird_person_character
                (:Is%20Valid
                  (Animation|PlayAnimMontage _asthird_person_character (Variables|Default|GetCharacter%20Shot%20Montage) 1.0 "None")))))
          (else
            (goto _label)))
        ;;[1 1 1] Play Wepon Animation
        (Components|Animation|PlayAnimation (Variables|Default|GetSkeletalMesh) (Variables|Default|GetWeapon%20Shot%20Animation) false)
        ;;[1 1 1] Spawn Shot Sound
        (Audio|SpawnSoundAttached (Variables|Default|GetShot%20Sound) (Variables|Default|GetItem%20Mesh) "None" "0, 0, 0" "0, 0, 0" "KeepRelativeOffset" false 1.0 1.0 0.0 "/Game/UltimateSurvivalPack/Blueprints/Attenuation/SA_Shot.SA_Shot" 0)
        (Effects|SpawnEmitterAttached "/Game/UltimateSurvivalPack/Demo/Particles/P_TriggerFire.P_TriggerFire" (Variables|Default|GetTrigger) "None"))
      ;[1 1 1] Spawn Splash
      (if (Math|Boolean|NORBoolean (Class|KismetMathLibrary|EqualExactlyVectorVector Water%20Hit "0, 0, 0") (Class|KismetMathLibrary|EqualExactlyVectorVector Water%20Hit "1.000000,1.000000,1.000000"))
        (Niagara|SpawnSystematLocation "/Game/UltimateSurvivalPack/Demo/Particles/Niagara/NS_WaterSplash_Small.NS_WaterSplash_Small" Water%20Hit)
        (Audio|SpawnSoundatLocation "/Game/UltimateSurvivalPack/Demo/Audio/Impact/CUE_WaterHit_01.CUE_WaterHit_01" Water%20Hit "0, 0, 0" 1.0 1.0 0.0 "/Game/UltimateSurvivalPack/Blueprints/Attenuation/SA_Footsteps.SA_Footsteps" 0))
      ;[1 1 1] Spawn Hit Effect
      (if Bullet%20Hit
        (Utilities|Casting|CastToSkeletalMeshComponent _hitcomponent_2
          (:then
            (Niagara|SpawnSystematLocation "/Game/UltimateSurvivalPack/Demo/Particles/Niagara/NS_BloodSplash.NS_BloodSplash" _impactpoint_2))
          (:CastFailed
            ;;[1 1 1] Spawn Bullet Decal
            (bind _returnvalue_2 (Class|GameplayStatics|SpawnDecalAttached "/Game/UltimateSurvivalPack/Material/M_BulletHole.M_BulletHole" "3.000000,3.000000,3.000000" _hitcomponent_2 "None" _impactpoint_2 (Math|Conversions|RotationFromXVector _impactnormal_2) "KeepWorldPosition" 3e+01))
            (Utilities|IsValid _returnvalue_2
              (:Is%20Valid
                (Rendering|Components|Decal|SetFadeOut _returnvalue_2 25.0 1.0 false)
                (Rendering|Components|Decal|SetFadeScreenSize _returnvalue_2 0.0015))
              (:Is%20Not%20Valid
                _))
            (if (Class|KismetMathLibrary|EqualExactlyVectorVector Water%20Hit "0, 0, 0")
              (Effects|SpawnEmitteratLocation "/Game/UltimateSurvivalPack/Demo/Particles/P_ImpactSmoke.P_ImpactSmoke" _impactpoint_2)
              (Audio|SpawnSoundatLocation "/Game/UltimateSurvivalPack/Demo/Audio/Impact/CUE_BulletImpact.CUE_BulletImpact" _impactpoint_2 "0, 0, 0" 0.25 1.0 0.0 "/Game/UltimateSurvivalPack/Blueprints/Attenuation/SA_Footsteps.SA_Footsteps" 0))))))
    (else
      ;;[1 1 1] Spawn Empty Shot Sound
      (Audio|SpawnSoundAttached (Variables|Default|GetClick%20Sound) (Variables|Default|GetItem%20Mesh) "None" "0, 0, 0" "0, 0, 0" "KeepRelativeOffset" false 1.0 1.0 0.0 "/Game/UltimateSurvivalPack/Blueprints/Attenuation/SA_Footsteps.SA_Footsteps" 0))))

(fn GetDamage
  (params (Hit :type Hit%20Result%20Structure%20%28by%20ref%29))
  (return (* (|CallParentFunction Hit) (- 1.0 (Math|Float|Clamp(Float) (/ (- (Math|Vector|Distance(Vector) (.ImpactPoint (Collision|BreakHitResult Hit)) (Transformation|GetActorLocation)) 5e+02) 3.5e+03) 0.1)))))