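; Sniper rifle holdable weapon that replaces standard aiming with a scope view.
; Aiming in third person blends to a runtime-created camera on a capsule-attached spring arm that follows control rotation, while first person changes the character's FOV.
; Both modes hide the character and rifle and show a scope widget, undone on un-aim or local destruction.
; Fire-mode and close-aim events are empty overrides, and toggling upgrade mode while not aiming destroys the aim camera.
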(event EventTick
  (params (DeltaSeconds :type Float%20%28single-precision%29))
  ;[1 0.2422 0.1625] Sniper aiming
  ;;[1 1 1] On tick update camera control rot
  (|CallParentFunction DeltaSeconds)
  (if (CallFunction|IsOwnerLocal)
    (Transformation|SetWorldRotation (Variables|Default|GetSpringArm) (Pawn|GetControlRotation (Game|GetPlayerController 0) :!class /Script/Engine.Controller) false false)))

(event EventAimingAction
  (params (Toggle :type Boolean))
  (bind _returnvalue (Game|GetPlayerController 0))
  (bind _springarm (Variables|Default|GetSpringArm))
  (bind _human_player_character (CallFunction|GetHumanPlayerCharacter _returnvalue))
  ;[1 0.2422 0.1625] Sniper aiming
  (if (not (Variables|Default|GetUpgrade%20Mode))
    (|CallParentFunction Toggle)
    (if Toggle
      (if (not (CallFunction|IsFirstPerson))
        (Variables|Default|GetAim%20Camera
          (:then
            _)
          (:else
            (bind _returnvalue_2 (AddComponent|AddCameraComponent false))
            (bind _output_get (Variables|Default|SetAim%20Camera _returnvalue_2))
            (Transformation|AttachComponentToComponent _output_get (Variables|Default|GetSpringArm) "None" "KeepRelative" "KeepRelative" "KeepRelative" true)))
        ;;[1 1 1] Adjust camera
        (Transformation|AttachComponentToComponent _springarm (Variables|/Script/Engine.Character|GetCapsuleComponent _human_player_character) "" "KeepRelative" "KeepRelative" "KeepRelative" true)
        (Transformation|SetRelativeLocation _springarm "0.000000,0.000000,60.000000" false false)
        ;;[1 1 1] Blend camera
        (Game|Player|SetViewTargetwithBlend (Game|GetPlayerController 0) self 0.3 "VTBlend_Linear" 1.0 false)
        (else
          (bind _asthird_person_character (Utilities|Casting|CastToThirdPersonCharacter (Variables|Default|GetInstigator)))
          (Default|UpdateFOV _asthird_person_character 15.0)))
      ;;[1 1 1] Adjust visibility
      (Development|SetHiddeninGame (Variables|/Script/Engine.Character|GetMesh _human_player_character) true true)
      (Development|SetHiddeninGame (Variables|Default|GetSkeletalMesh) true false)
      ;;[1 1 1] Remove scope widget
      (bind _scope_widget (Variables|Default|GetScope%20Widget)
        (:then
          (Widget|RemovefromParent _scope_widget))
        (:else
          _))
      ;;[1 1 1] Create scope widget
      (bind _returnvalue_3 (UserInterface|CreateWidget "/Game/UltimateSurvivalPack/Widget/W_Scope.W_Scope_C"))
      (bind _output_get_2 (Variables|Default|SetScope%20Widget _returnvalue_3))
      (UserInterface|Viewport|AddtoViewport _output_get_2 -1)
      (else
        (bind _asthird_person_character_2 (Utilities|Casting|CastToThirdPersonCharacter (Variables|Default|GetInstigator)))
        (Default|UpdateFOV _asthird_person_character_2 0.0)
        ;;[1 1 1] Blend camera
        (Game|Player|SetViewTargetwithBlend (Game|GetPlayerController 0) (CallFunction|GetHumanPlayerCharacter (Game|GetPlayerController 0)) 0.3 "VTBlend_Linear" 0.3 false)
        ;;[1 1 1] Reset visibility
        (Development|SetHiddeninGame (Variables|/Script/Engine.Character|GetMesh (CallFunction|GetHumanPlayerCharacter (Game|GetPlayerController 0))) false true)
        (Development|SetHiddeninGame (Variables|Default|GetSkeletalMesh) false true)
        ;;[1 1 1] Remove scope widget
        (bind _scope_widget_2 (Variables|Default|GetScope%20Widget)
          (:then
            (Widget|RemovefromParent _scope_widget_2))
          (:else))))))

(event EventChangeFiremode)

(event EventDestroyed
  ;[1 0.2422 0.1625] Sniper aiming
  ;;[1 1 1] On Destroyed
  (|CallParentFunction)
  (if (CallFunction|IsOwnerLocal)
    (if (and (Utilities|IsValid (Game|GetPlayerController 0)) (Utilities|IsValid (CallFunction|GetHumanPlayerCharacter (Game|GetPlayerController 0))))
      (bind _asthird_person_character (Utilities|Casting|CastToThirdPersonCharacter (Variables|Default|GetInstigator)))
      (Default|UpdateFOV _asthird_person_character 0.0)
      ;;[1 1 1] Blend camera
      (Game|Player|SetViewTargetwithBlend (Game|GetPlayerController 0) (CallFunction|GetHumanPlayerCharacter (Game|GetPlayerController 0)) 0.3 "VTBlend_Linear" 0.3 false)
      ;;[1 1 1] Reset visibility
      (Development|SetHiddeninGame (Variables|/Script/Engine.Character|GetMesh (CallFunction|GetHumanPlayerCharacter (Game|GetPlayerController 0))) false true)
      (Development|SetHiddeninGame (Variables|Default|GetSkeletalMesh) false true)
      ;;[1 1 1] Remove scope widget
      (bind _scope_widget (Variables|Default|GetScope%20Widget)
        (:then
          (Widget|RemovefromParent _scope_widget))
        (:else)))))

(event EventCloseAiming
  ;[1 0.2422 0.1625] Sniper aiming
)

(fn ConstructionScript
  (|CallParentFunction))

(fn ToggleUpgradeMode
  (params (Toggle :type Boolean))
  (if (CallFunction|IsOwnerLocal)
    (if (not (Variables|Default|GetIs%20Aiming))
      (bind _aim_camera (Variables|Default|GetAim%20Camera)
        (:then
          (Components|DestroyComponent _aim_camera))
        (:else
          _))
      (|CallParentFunction Toggle))))