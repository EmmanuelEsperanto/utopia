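; Holdable wrench that lets players repair buildings and shows the cupboard zones they have privilege in while it is equipped.
; For the local owner, a camera sphere trace each Tick shows a repair widget for non-harvestable actors with a building component.
; Holding primary action plays the widget's fill animation on a timer of equal length, repeating a server repair on each completion.
; The server repairs if no cupboard is registered or the player has privilege.
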(event Custom|Toggle%20Time
  (params (Toggle :type Boolean))
  (bind _repair_widget (Variables|Default|GetRepair%20Widget))
  (Utilities|IsValid (Variables|Default|GetRepair%20Widget)
    (:Is%20Valid
      (if Toggle
        (Default|PlayAnimation _repair_widget)
        (if (not (Utilities|Time|IsValidTimerHandle (Variables|Default|GetTimer)))
          (bind _returnvalue (Utilities|Time|SetTimerbyEvent (delegate Custom|Repair%20Building) (Class|WidgetAnimation|GetEndTime (Variables|/Game/UltimateSurvivalPack/Widget/W_WrenchInformation.W_WrenchInformation_C|GetFillAnimation _repair_widget))))
          (Variables|Default|SetTimer _returnvalue))
        (else
          (Default|StopAnimation (Variables|Default|GetRepair%20Widget))
          (if (Utilities|Time|IsValidTimerHandle (Variables|Default|GetTimer))
            (Utilities|Time|ClearandInvalidateTimerbyHandle (Variables|Default|GetTimer))))))))

(event Custom|Repair%20Building
  (CallFunction|SERVERRepair (.HitActor (Collision|BreakHitResult (Variables|Default|GetHit))))
  (CallFunction|ToggleTime false)
  (CallFunction|ToggleTime true))

(event Custom|SERVER%20Destroy%20Building
  (params (Destroy%20Building :type Actor%20Object%20Reference))
  (Utilities|IsValid Destroy%20Building
    (:Is%20Valid
      (Actor|DestroyActor Destroy%20Building))))

(event Custom|SERVER%20Repair
  (params (Target :type Actor%20Object%20Reference))
  (bind _returnvalue (Actor|GetComponentbyClass Target "/Game/UltimateSurvivalPack/Blueprints/Buildings/Parent/BP_BuildingComponent.BP_BuildingComponent_C"))
  (bind _assurvival_gamemode (Utilities|Casting|CastToSurvivalGamemode (Game|GetGameMode)))
  (if (.ReturnValue (Utilities|Map|Find (Variables|/Game/UltimateSurvivalPack/Blueprints/SurvivalGamemode.SurvivalGamemode_C|GetBuilding%20Actors _assurvival_gamemode) (Variables|/Game/UltimateSurvivalPack/Blueprints/Buildings/Parent/BP_BuildingComponent.BP_BuildingComponent_C|GetCupboard%20ID _returnvalue)))
    (bind _asbp_cupboard (Utilities|Casting|CastToBP_Cupboard (.Value (Utilities|Map|Find (Variables|/Game/UltimateSurvivalPack/Blueprints/SurvivalGamemode.SurvivalGamemode_C|GetBuilding%20Actors _assurvival_gamemode) (Variables|/Game/UltimateSurvivalPack/Blueprints/Buildings/Parent/BP_BuildingComponent.BP_BuildingComponent_C|GetCupboard%20ID _returnvalue)))))
    (if (Utilities|Array|ContainsItem (Variables|/Game/UltimateSurvivalPack/Blueprints/Buildings/Final/BP_Cupboard.BP_Cupboard_C|GetPrivilege%20Players _asbp_cupboard) (Variables|/Game/UltimateSurvivalPack/Blueprints/Components/BP_PlayerComponent.BP_PlayerComponent_C|GetPlayer%20Unique%20ID (CallFunction|GetPlayerComponent (Variables|Default|GetInstigator))))
      (Default|SERVERRepair _returnvalue self :!label _label))
    (else
      (goto _label))))

(event EventBeginPlay
  (bind _returnvalue (Components|GetOwner))
  (|CallParentFunction)
  ;[1 1 1] Is Local
  (Utilities|IsValid _returnvalue
    (:Is%20Valid
      (bind _ascontroller (Utilities|Casting|CastToController _returnvalue))
      (if (Pawn|IsLocalController _ascontroller)
        ;[1 1 1] Set Cupboard Zone Visibility
        (bind _outactors (Actor|GetAllActorsOfClass "/Game/UltimateSurvivalPack/Blueprints/Buildings/Final/BP_Cupboard.BP_Cupboard_C"))
        (for _array_element _outactors
          (if (Utilities|Array|ContainsItem (Variables|/Game/UltimateSurvivalPack/Blueprints/Buildings/Final/BP_Cupboard.BP_Cupboard_C|GetPrivilege%20Players _array_element) (Variables|/Game/UltimateSurvivalPack/Blueprints/Components/BP_PlayerComponent.BP_PlayerComponent_C|GetPlayer%20Unique%20ID (CallFunction|GetPlayerComponent (Variables|Default|GetInstigator))))
            (Rendering|SetVisibility (Variables|/Game/UltimateSurvivalPack/Blueprints/Buildings/Final/BP_Cupboard.BP_Cupboard_C|GetZone _array_element) true false)))))))

(event EventTick
  (params (DeltaSeconds :type Float%20%28single-precision%29))
  (bind _returnvalue (Game|GetPlayerCameraManager 0))
  (bind _timer (Variables|Default|GetTimer))
  (bind _returnvalue_2 (Camera|GetCameraLocation _returnvalue))
  (if (CallFunction|IsOwnerLocal)
    (bind (_outhit _returnvalue_3) (Collision|SphereTraceByChannel _returnvalue_2 (+ _returnvalue_2 (* (Math|Vector|GetForwardVector (Camera|GetCameraRotation _returnvalue)) (Variables|/Game/UltimateSurvivalPack/Blueprints/Components/BP_PlayerInventoryComponent.BP_PlayerInventoryComponent_C|GetInteraction%20Distance (CallFunction|GetInventoryComponent (Game|GetPlayerController 0))))) 3.0 "TraceTypeQuery1" true 0 "None"))
    (Variables|Default|SetHit _outhit)
    (if _returnvalue_3
      (Utilities|IsValid (Actor|GetComponentbyClass (.HitActor (Collision|BreakHitResult _outhit)) "/Game/UltimateSurvivalPack/Blueprints/Buildings/Parent/BP_BuildingComponent.BP_BuildingComponent_C")
        (:Is%20Valid
          (Utilities|Casting|CastToBP_Harvestable (.HitActor (Collision|BreakHitResult _outhit))
            (:then
              (Utilities|IsValid (Variables|Default|GetRepair%20Widget) :!label _label
                (:Is%20Valid
                  (Widget|RemovefromParent (Variables|Default|GetRepair%20Widget))
                  (Variables|Default|SetRepair%20Widget 0)
                  (if (Utilities|Time|IsValidTimerHandle _timer)
                    (Utilities|Time|ClearandInvalidateTimerbyHandle _timer)))))
            (:CastFailed
              (Utilities|IsValid (Variables|Default|GetRepair%20Widget)
                (:Is%20Valid
                  (if (not (== (Actor|GetComponentbyClass (.HitActor (Collision|BreakHitResult _outhit)) "/Game/UltimateSurvivalPack/Blueprints/Buildings/Parent/BP_BuildingComponent.BP_BuildingComponent_C") (Variables|/Game/UltimateSurvivalPack/Widget/W_WrenchInformation.W_WrenchInformation_C|GetBuilding%20Component (Variables|Default|GetRepair%20Widget))))
                    (Widget|RemovefromParent (Variables|Default|GetRepair%20Widget))
                    (bind _returnvalue_4 (UserInterface|CreateWidget "/Game/UltimateSurvivalPack/Widget/W_WrenchInformation.W_WrenchInformation_C" 0 (Actor|GetComponentbyClass (.HitActor (Collision|BreakHitResult _outhit)) "/Game/UltimateSurvivalPack/Blueprints/Buildings/Parent/BP_BuildingComponent.BP_BuildingComponent_C") :!label _label_2))
                    (bind _output_get (Variables|Default|SetRepair%20Widget _returnvalue_4))
                    (UserInterface|Viewport|AddtoViewport _output_get 0)))
                (:Is%20Not%20Valid
                  (goto _label_2))))))
        (:Is%20Not%20Valid
          (goto _label)))
      (else
        (goto _label)))))

(event EventDestroyed
  (bind _returnvalue (Components|GetOwner))
  (Utilities|IsValid (Variables|Default|GetRepair%20Widget)
    (:Is%20Valid
      (Widget|RemovefromParent (Variables|Default|GetRepair%20Widget))
      (Variables|Default|SetRepair%20Widget 0))
    (:Is%20Not%20Valid
      _))
  (Utilities|IsValid _returnvalue
    (:Is%20Valid
      (bind _ascontroller (Utilities|Casting|CastToController _returnvalue))
      (if (Pawn|IsLocalController _ascontroller)
        ;[1 1 1] Set Cupboard Zone Visibility
        (bind _outactors (Actor|GetAllActorsOfClass "/Game/UltimateSurvivalPack/Blueprints/Buildings/Final/BP_Cupboard.BP_Cupboard_C"))
        (for _array_element _outactors
          (if (Utilities|Array|ContainsItem (Variables|/Game/UltimateSurvivalPack/Blueprints/Buildings/Final/BP_Cupboard.BP_Cupboard_C|GetPrivilege%20Players _array_element) (Variables|/Game/UltimateSurvivalPack/Blueprints/Components/BP_PlayerComponent.BP_PlayerComponent_C|GetPlayer%20Unique%20ID (CallFunction|GetPlayerComponent (Variables|Default|GetInstigator))))
            (Rendering|SetVisibility (Variables|/Game/UltimateSurvivalPack/Blueprints/Buildings/Final/BP_Cupboard.BP_Cupboard_C|GetZone _array_element) false false)))))))

(event EventPrimaryAction
  (params (Pressed :type Boolean))
  (CallFunction|ToggleTime Pressed))

(fn ConstructionScript
  (|CallParentFunction))