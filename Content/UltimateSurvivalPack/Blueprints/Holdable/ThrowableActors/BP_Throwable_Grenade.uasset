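; Throwable grenade actor that detonates after a fuse delay or when hit by point damage.
; On BeginPlay the authority starts the detonation timer, while non-explosion point damage jumps straight to detonation, so explosion damage does not trigger it.
; Both paths share a DoOnce that spawns a scaled-up BP_Explosion at the grenade's location, passing along owner and instigator, then destroys the grenade.
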(event EventBeginPlay
  (|CallParentFunction)
  (Networking|SwitchHasAuthority
    (:Authority
      ;[1 1 1] Wait For Detonation
      (Utilities|FlowControl|Delay (Variables|Default|GetDetonation%20Time))
      (Utilities|FlowControl|DoOnce false
        (:Completed
          ;[1 1 1] Spawn Explosion Actor
          (Game|SpawnActorfromClass "/Game/UltimateSurvivalPack/Blueprints/Holdable/Others/BP_Explosion.BP_Explosion_C" (Math|Transform|MakeTransform (Transformation|GetActorLocation) "0, 0, 0" "4.000000,4.000000,4.000000") "Undefined" (Components|GetOwner) (Variables|Default|GetInstigator))
          ;[1 1 1] Destroy Self
          (Actor|DestroyActor))))))

(event Game|Damage|EventPointDamage
  (params (Damage :type Float%20%28single-precision%29) (DamageType :type Damage%20Type%20Object%20Reference) (HitLocation :type Vector :default "0, 0, 0") (HitNormal :type Vector :default "0, 0, 0") (HitComponent :type Primitive%20Component%20Object%20Reference) (BoneName :type Name :default "None") (ShotFromDirection :type Vector :default "0, 0, 0") (InstigatedBy :type Controller%20Object%20Reference) (DamageCauser :type Actor%20Object%20Reference) (HitInfo :type Hit%20Result%20Structure%20%28by%20ref%29))
  ;[1 1 1] Explode Grenade after receiving Point Damage
  ;;[1 1 1] Filter Explosion Damage
  (if (!= (Utilities|GetClass DamageType) "/Game/UltimateSurvivalPack/Blueprints/DamageType/DT_Explosion.DT_Explosion_C")
    (Utilities|FlowControl|DoOnce false
      (:Completed
        ;[1 1 1] Spawn Explosion Actor
        (Game|SpawnActorfromClass "/Game/UltimateSurvivalPack/Blueprints/Holdable/Others/BP_Explosion.BP_Explosion_C" (Math|Transform|MakeTransform (Transformation|GetActorLocation) "0, 0, 0" "4.000000,4.000000,4.000000") "Undefined" (Components|GetOwner) (Variables|Default|GetInstigator))
        ;[1 1 1] Destroy Self
        (Actor|DestroyActor)))))

(fn ConstructionScript
  (|CallParentFunction))