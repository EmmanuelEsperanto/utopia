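; Lobby player controller that handles input for emotes, pod overview and server save deletion.
; It forwards a random dance toggle, pod selection on mouse release and per-tick rotation input to BPLobbyComponent, whose HUD also supplies the chat widget.
; With authority, Delete uses a FlipFlop as two-press confirmation to wipe the PlayerSave slot and give the game instance a fresh save object, reporting through BPOnlineComponent chat messages.
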(event EventTick
  (params (DeltaSeconds :type Float%20%28single-precision%29))
  ;[1 1 1] Mouse Character Rotation Input
  (|CallParentFunction DeltaSeconds)
  (Default|UpdateOverviewingPodRotation (Variables|Default|GetBP_LobbyComponent) (Class|Actor|GetInputAxisKeyValue)))

(event Input|MouseEvents|LeftMouseButton
  (params (Key :type Key%20Structure :default "None"))
  ;[0.5113 1 0.2222] Input
  ;;[1 1 1] Pod Overview Input
  (:Released
    (Default|UpdateOverviewingPod (Variables|Default|GetBP_LobbyComponent))))

(event Input|KeyboardEvents|E
  (params (Key :type Key%20Structure :default "None"))
  ;[0.5113 1 0.2222] Input
  ;;[1 1 1] Toggle Dance
  (:Pressed
    (Default|ToggleDance (Variables|Default|GetBP_LobbyComponent) (.OutItem (Utilities|Array|Random (Variables|/Game/UltimateSurvivalPack/LobbySystem/Blueprints/BP_LobbyComponent.BP_LobbyComponent_C|GetEmotes (Variables|Default|GetBP_LobbyComponent)))))))

(event Input|KeyboardEvents|Delete
  (params (Key :type Key%20Structure :default "None"))
  ;[0.5113 1 0.2222] Input
  ;;[1 1 1] Delete server save
  (:Pressed
    (if (Ability|HasAuthority)
      (Utilities|Casting|CastToBP_GameInstance_UMSP (Game|GetGameInstance))
      (bind _returnvalue (SaveGame|DoesSaveGameExist "PlayerSave"))
      (if _returnvalue
        (Utilities|FlowControl|FlipFlop
          (:A
            (Default|CLIENTReceiveChatMessage (Variables|Default|GetBP_OnlineComponent) "SAVING SYSTEM" "WARNING! You are about to delete all of your server saved data. Do you really want to proceed? If YES, click [ DEL ]" "(R=1.000000,G=0.763893,B=0.196295,A=1.000000)"))
          (:B
            (bind _returnvalue_2 (SaveGame|DeleteGameinSlot "PlayerSave"))
            (if _returnvalue_2
              (bind _asbp_game_instance_umsp (Utilities|Casting|CastToBP_GameInstance_UMSP (Game|GetGameInstance)))
              (bind _returnvalue_3 (SaveGame|CreateSaveGameObject "/Game/UltimateSurvivalPack/Blueprints/Save/SAV_ServerData.SAV_ServerData_C"))
              (Variables|/Game/UltimateSurvivalPack/Blueprints/BP_GameInstance_UMSP.BP_GameInstance_UMSP_C|SetPlayer%20Save _asbp_game_instance_umsp _returnvalue_3)
              (Default|CLIENTReceiveChatMessage (Variables|Default|GetBP_OnlineComponent) "SAVING SYSTEM" "Successfully deleted server save data!" "(R=0.058054,G=1.000000,B=0.102191,A=1.000000)"))))
        (else
          (Default|CLIENTReceiveChatMessage (Variables|Default|GetBP_OnlineComponent) "SAVING SYSTEM" "You do not have any server save." "(R=0.334474,G=0.808100,B=1.000000,A=1.000000)"))))))

(fn ConstructionScript)

(fn GetChatWidget
  (return (Variables|/Game/UltimateSurvivalPack/LobbySystem/Widget/W_LobbyMenu.W_LobbyMenu_C|GetW_Chat (Variables|/Game/UltimateSurvivalPack/LobbySystem/Blueprints/BP_LobbyComponent.BP_LobbyComponent_C|GetHUD (Variables|Default|GetBP_LobbyComponent)))))