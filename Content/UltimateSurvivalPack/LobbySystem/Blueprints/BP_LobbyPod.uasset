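; Lobby pod actor that displays one player's character, with name, ready state, backlight and emotes, or an invite widget when empty.
; Modular body meshes follow the main mesh via master pose, with customization applied through meshes and a dynamic material.
; Player data rebuilds socketed holsters and sets gendered armor from a data table, hiding parts under headgear.
; Clicking reports the pod to the lobby component; a timeline handles turning and eased return.
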(event OnClicked(MouseCollision)
  (params (TouchedComponent :type Primitive%20Component%20Object%20Reference) (ButtonPressed :type Key%20Structure))
  ;[1 0.6162 0.08689] Update Character Rotation
  ;;[1 1 1] On Lobby pod clicked
  ;;;[1 1 1] Worth to rotate
  (if (and (Variables|Non-Editable|GetIs%20Occupied) (Variables|PodSettings|GetCan%20Rotate%20Player))
    ;;;[1 1 1] Update references in Component and start update timeline
    (Default|UpdateOverviewingPod (CallFunction|GetLobbyComponent (Game|GetPlayerController 0)) self)
    (CallFunction|StartUpdateActorRotation)))

(event Custom|Load%20Pod
  (params (Player%20Name :type String) (Unique%20ID :type String) (Is%20Ready :type Boolean))
  ;[0.3032 1 0.1758] Load Pod
  ;;[1 1 1] Occupie Pod
  (CallFunction|OccupiePod true)
  ;;[1 1 1] Save Player ID and Name
  (bind _output_get (Variables|Non-Editable|SetPlayer%20Unique%20ID Unique%20ID))
  (bind _output_get_2 (Variables|Non-Editable|SetPlayer%20Name Player%20Name))
  ;;[1 1 1] Load Player Information Widget
  (CallFunction|LoadPlayerWidgetInformation _output_get_2 _output_get)
  (CallFunction|ToggleReady Is%20Ready)
  (CallFunction|TogglePodLight false "(R=1.000000,G=1.000000,B=1.000000,A=1.000000)") ; Turn off light to prevent any light glitch
)

(event Custom|Load%20Player%20Widget%20Information
  (params (Player%20Name :type String) (Unique%20ID :type String))
  ;[1 1 1] Update Player Widget
  (bind _asw_lobby_info (Utilities|Casting|CastToW_LobbyInfo (UserInterface|GetUserWidgetObject (Variables|Default|GetPlayer%20Info))))
  (Default|LoadPlayerInformation _asw_lobby_info Player%20Name Unique%20ID))

(event Custom|Start%20Update%20Actor%20Rotation
  (bind _charactermesh (Variables|Default|GetCharacterMesh))
  (bind _charactermesh_2 (Variables|Default|GetCharacterMesh))
  (bind _relativerotation (Variables|/Script/Engine.SceneComponent|GetRelativeRotation _charactermesh_2))
  (bind _relativerotation_2 (Variables|/Script/Engine.SceneComponent|GetRelativeRotation _charactermesh))
  ;[1 0.6162 0.08689] Update Character Rotation
  ;;[1 1 1] Start / Reverse the update
  (Audio|Components|Audio|Stop (Variables|Default|GetTML%20Actor%20Rotation))
  (bind _direction (Timeline|TML%20Actor%20Rotation PlayFromStart)
    (:Update
      (switch Utilities|FlowControl|Switch|SwitchonETimelineDirection _direction
        (:Forward
          ;;[1 1 1] Rotate character to depending turn rotation desired by X look input
          (if (not (Math|Float|NearlyEqual(Float) (Variables|Non-Editable|GetTurn%20Value) 0.0 0.1))
            (Transformation|SetRelativeRotation (Variables|Default|GetCharacterMesh) (Math|Rotator|MakeRotator 0.0 0.0 (Math|Interpolation|FInterpTo (.yaw _relativerotation_2) (+ (Variables|Non-Editable|GetTurn%20Value) (.yaw _relativerotation_2)) (Utilities|Time|GetWorldDeltaSeconds) 1e+01)) false false)))
        (:Backward
          ;;[1 1 1] Smoothly update Character to default Rotation
          (if (Math|Float|NearlyEqual(Float) (.yaw _relativerotation) 9e+01 1.0)
            (Audio|Components|Audio|Stop (Variables|Default|GetTML%20Actor%20Rotation))
            (else
              (Transformation|SetRelativeRotation (Variables|Default|GetCharacterMesh) (Math|Rotator|MakeRotator 0.0 0.0 (.yaw (Math|Rotator|Lerp(Rotator) (Math|Rotator|MakeRotator 0.0 0.0 (.yaw _relativerotation)) "0,90.000000, 0" 0.1 true))) false false))))))))

(event Custom|Update%20Turn%20Value
  (params (Mouse%20X :type Float%20%28double-precision%29))
  ;[1 0.6162 0.08689] Update Character Rotation
  ;;[1 1 1] Update Turn Value
  (Variables|Non-Editable|SetTurn%20Value (* Mouse%20X 45.0)))

(event Custom|Load%20Player%20Data
  (params (Player%20Data :type S%20Player%20Save%20Structure))
  (bind (_armor _holsterdata) (Utilities|Struct|BreakS_PlayerSave Player%20Data))
  (Variables|Default|SetPlayer%20Data Player%20Data)
  ;[1 1 1] Destroy Old Component
  (for _array_element (Variables|Default|GetHolster%20References)
    (Components|DestroyComponent _array_element))
  ;[1 1 1] Create Holsters
  (for _array_element_2 _holsterdata
    (CallFunction|CreateHolster _array_element_2))
  ;[1 1 1] Apply Armor
  (CallFunction|ApplyArmor _armor))

(event Custom|Occupie%20Pod
  (params (Occupied :type Boolean))
  ;[1 0.02604 0.02604] Occupie Pod
  (bind _output_get (Variables|Non-Editable|SetIs%20Occupied Occupied))
  (Rendering|SetVisibility (Variables|Default|GetPlayer%20Info) _output_get false)
  (Rendering|SetVisibility (Variables|Default|GetInvite%20Widget) (not _output_get) false))

(event Custom|Toggle%20Ready
  (params (Ready :type Boolean))
  ;[0.1511 0.5841 1] Toggle Ready
  (bind _asw_lobby_info (Utilities|Casting|CastToW_LobbyInfo (UserInterface|GetUserWidgetObject (Variables|Default|GetPlayer%20Info))))
  (Default|ToggleReady _asw_lobby_info Ready))

(event Custom|Remove%20Pod
  ;[1 0.25 0.25] Remove Pod
  ;;[1 1 1] Occupie Pod
  (CallFunction|OccupiePod false)
  ;;[1 1 1] Null values
  (Variables|Non-Editable|SetPlayer%20Unique%20ID "")
  (Variables|Non-Editable|SetPlayer%20Name ""))

(event Custom|Toggle%20Pod%20Light
  (params (Toggle :type Boolean) (Color :type Linear%20Color%20Structure :default "(R=1.000000,G=1.000000,B=1.000000,A=1.000000)"))
  (bind _pointlight (Variables|Default|GetPointLight))
  ;[1 1 1] Toggle pod backlight
  (Rendering|SetVisibility _pointlight Toggle false)
  (Rendering|Components|Light|SetLightColor _pointlight Color true)
  (Rendering|SetVisibility (Variables|Default|GetShine%20Mesh) Toggle false)
  (Rendering|Material|SetVectorParameterValue (Variables|Non-Editable|GetShine%20Material) "Color" Color :!class /Script/Engine.MaterialInstanceDynamic))

(event Custom|Toggle%20Dance
  (params (Emote :type Anim%20Montage%20Object%20Reference))
  (bind _charactermesh (Variables|Default|GetCharacterMesh))
  (bind _returnvalue (Components|SkeletalMesh|GetAnimInstance _charactermesh))
  ;[1 1 1] Set Dance Index To AnimBP | 0 = Idle
  (if (Class|AnimInstance|IsAnyMontagePlaying _returnvalue)
    (Animation|Montage|MontageStop _returnvalue 0.5 0)
    (else
      (Animation|Montage|PlayMontage (Variables|Default|GetCharacterMesh) Emote))))

(event Custom|Toggle%20Selected
  (params (Toggle :type Boolean))
  ;[1 1 1] Toggle Selected
  (CallFunction|TogglePodLight Toggle "(R=1.000000,G=0.200000,B=0.200000,A=1.000000)"))

(event Custom|Return%20Default%20Rotation
  (bind _charactermesh (Variables|Default|GetCharacterMesh))
  (bind _charactermesh_2 (Variables|Default|GetCharacterMesh))
  (bind _relativerotation (Variables|/Script/Engine.SceneComponent|GetRelativeRotation _charactermesh_2))
  (bind _relativerotation_2 (Variables|/Script/Engine.SceneComponent|GetRelativeRotation _charactermesh))
  ;[1 0.6162 0.08689] Update Character Rotation
  ;;[1 1 1] Start / Reverse the update
  (Audio|Components|Audio|Stop (Variables|Default|GetTML%20Actor%20Rotation))
  (bind _direction (Timeline|TML%20Actor%20Rotation ReverseFromEnd)
    (:Update
      (switch Utilities|FlowControl|Switch|SwitchonETimelineDirection _direction
        (:Forward
          ;;[1 1 1] Rotate character to depending turn rotation desired by X look input
          (if (not (Math|Float|NearlyEqual(Float) (Variables|Non-Editable|GetTurn%20Value) 0.0 0.1))
            (Transformation|SetRelativeRotation (Variables|Default|GetCharacterMesh) (Math|Rotator|MakeRotator 0.0 0.0 (Math|Interpolation|FInterpTo (.yaw _relativerotation_2) (+ (Variables|Non-Editable|GetTurn%20Value) (.yaw _relativerotation_2)) (Utilities|Time|GetWorldDeltaSeconds) 1e+01)) false false)))
        (:Backward
          ;;[1 1 1] Smoothly update Character to default Rotation
          (if (Math|Float|NearlyEqual(Float) (.yaw _relativerotation) 9e+01 1.0)
            (Audio|Components|Audio|Stop (Variables|Default|GetTML%20Actor%20Rotation))
            (else
              (Transformation|SetRelativeRotation (Variables|Default|GetCharacterMesh) (Math|Rotator|MakeRotator 0.0 0.0 (.yaw (Math|Rotator|Lerp(Rotator) (Math|Rotator|MakeRotator 0.0 0.0 (.yaw _relativerotation)) "0,90.000000, 0" 0.1 true))) false false))))))))

(event Custom|Apply%20Customization
  (params (Customization%20Data :type S%20Player%20Customization%20Structure))
  (bind _human_dynamic_material (Variables|Default|GetHuman%20Dynamic%20Material))
  ;[1 1 1] Apply Customization To Player
  (Rendering|Material|SetVectorParameterValue _human_dynamic_material "Skin Color" (.skincolor Customization%20Data) :!class /Script/Engine.MaterialInstanceDynamic)
  (Rendering|Material|SetVectorParameterValue _human_dynamic_material "Stubble Color" (.stubblecolor Customization%20Data) :!class /Script/Engine.MaterialInstanceDynamic)
  (Rendering|Material|SetVectorParameterValue _human_dynamic_material "Hair Color" (.haircolor Customization%20Data) :!class /Script/Engine.MaterialInstanceDynamic)
  (Class|SkinnedMeshComponent|SetSkeletalMesh (Variables|Default|GetHair) (.hairmesh Customization%20Data) true)
  (Class|SkinnedMeshComponent|SetSkeletalMesh (Variables|Default|GetEyes) (.eyesmesh Customization%20Data) true)
  (Class|SkinnedMeshComponent|SetSkeletalMesh (Variables|Default|GetBeard) (.beardmesh Customization%20Data) true)
  (Class|SkinnedMeshComponent|SetSkeletalMesh (Variables|Default|GetEyebrows) (.eyebrows Customization%20Data) true)
  (bind _output_get (Variables|Default|SetGender%20Type (.gendertype Customization%20Data)))
  (Class|SkinnedMeshComponent|SetSkeletalMesh (Variables|Default|GetCharacterMesh) (CallFunction|GetGenderBody _output_get) false))

(event EventBeginPlay
  ;[1 0.5815 0.121] Begin Play
  ;[1 1 1] Set Invite Widget Referenced to pod for Hover Light Efect
  (bind _asw_invite_plus_button (Utilities|Casting|CastToW_InvitePlusButton (UserInterface|GetUserWidgetObject (Variables|Default|GetInvite%20Widget))))
  (Variables|/Game/UltimateSurvivalPack/LobbySystem/Widget/W_InvitePlusButton.W_InvitePlusButton_C|SetPod%20Reference _asw_invite_plus_button self))

(fn ConstructionScript
  (bind _returnvalue (Rendering|Material|CreateDynamicMaterialInstance (Variables|Default|GetShine%20Mesh) 0 "/Game/UltimateSurvivalPack/LobbySystem/Material/M_Shine.M_Shine" "None" :!class /Script/Engine.PrimitiveComponent))
  (Variables|Non-Editable|SetShine%20Material _returnvalue)
  ;[1 1 1] Create Dynamic Material
  (bind _returnvalue_2 (Rendering|Material|CreateDynamicMaterialInstance "/Game/UltimateSurvivalPack/Demo/Character/Material/M_Human.M_Human" "None" "None" :!class /Script/Engine.KismetMaterialLibrary))
  (Variables|Default|SetHuman%20Dynamic%20Material _returnvalue_2)
  ;[1 1 1] Set Masterpose
  (Class|SkinnedMeshComponent|SetMasterPoseComponent (Variables|Default|GetEyebrows) (Variables|Default|GetCharacterMesh) false)
  ;[1 1 1] Set Dynamic Material
  (Rendering|Material|SetMaterial (Variables|Default|GetCharacterMesh) 0 (Variables|Default|GetHuman%20Dynamic%20Material)))

(fn CreateHolster
  (params (Holster%20Data :type S%20Holster%20Data%20Structure))
  (bind (_holsterattachsocket _additivetransform _holsteractor) (Utilities|Struct|BreakS_HolsterData Holster%20Data))
  (bind (_holsterattachsocket_2 _additivetransform_2 _holstermesh) (Utilities|Struct|BreakS_HolsterData Holster%20Data))
  ;[1 0.5415 0.01729] Create Static Mesh or Actor?
  (if (not (Utilities|IsValidClass (Utilities|Struct|BreakS_HolsterData Holster%20Data)))
    ;[0 1 0.8061 1 75] Create Static Mesh Holster
    ;;[1 1 1] Create And Attach
    (bind _returnvalue (AddComponent|AddStaticMeshComponent false))
    (bind _output_get (LocalVariables|SetL%20Holster%20Reference _returnvalue))
    (Components|StaticMesh|SetStaticMesh _returnvalue _holstermesh)
    (Transformation|AttachComponentToComponent _output_get (Variables|Default|GetCharacterMesh) _holsterattachsocket_2 "SnapToTarget" "SnapToTarget" "KeepRelative" true)
    ;;[1 1 1] Add Additive Transform
    (Transformation|SetRelativeTransform _output_get _additivetransform_2 false false)
    (Utilities|Array|Add (Variables|Default|GetHolster%20References) (LocalVariables|GetL%20Holster%20Reference))
    (else
      ;[1 0.2887 0.2488 1 75] Create Child Actor Holster
      ;;[1 1 1] Create And Attach
      (bind _return (Class|BPIPlayer|CreateChildActorComponent(Message) (Components|GetOwner) _holsteractor))
      (bind _output_get_2 (LocalVariables|SetL%20Holster%20Reference _return))
      (Transformation|AttachComponentToComponent _output_get_2 (Variables|Default|GetCharacterMesh) _holsterattachsocket "SnapToTarget" "SnapToTarget" "KeepRelative" true)
      ;;;[1 1 1] Add Additive Transform
      (Transformation|SetRelativeTransform _output_get_2 _additivetransform false false)
      (Utilities|Array|Add (Variables|Default|GetHolster%20References) (LocalVariables|GetL%20Holster%20Reference)))))

(fn ApplyArmor
  (params (Armor :type S%20Player%20Armor%20Structure%20%28by%20ref%29))
  (bind (_headarmor _chestarmor _legsarmor _feetarmor) (Utilities|Struct|BreakS_PlayerArmor Armor))
  (for (_array_element _array_index) (Utilities|Array|MakeArray _headarmor _chestarmor _legsarmor _feetarmor)
    (bind _returnvalue (Utilities|GetDataTableRow "/Game/UltimateSurvivalPack/Blueprints/Datatable/Inventory/DT_ItemData.DT_ItemData" _array_element)
      (:then
        (LocalVariables|SetL%20Mesh (Utilities|Select :Index (Variables|Default|GetGender%20Type) :NewEnumerator0 (.ArmorMaleMesh (Utilities|Struct|BreakS_Item_ArmorProperties (.ArmorProperties (Utilities|Struct|BreakS_InventoryItemData _returnvalue)))) :NewEnumerator1 (.ArmorFemaleMesh (Utilities|Struct|BreakS_Item_ArmorProperties (.ArmorProperties (Utilities|Struct|BreakS_InventoryItemData _returnvalue))))))
        (switch int _array_index
          (:0
            (Class|SkinnedMeshComponent|SetSkeletalMesh (Variables|Default|GetHead) (LocalVariables|GetL%20Mesh) true)
            (for _array_element_2 (.HideMesh (Utilities|Struct|BreakS_Item_ArmorProperties (.ArmorProperties (Utilities|Struct|BreakS_InventoryItemData _returnvalue))))
              (Development|SetHiddeninGame (Utilities|Select :Index _array_element_2 :NewEnumerator0 (Variables|Default|GetHair) :NewEnumerator1 (Variables|Default|GetEyes) :NewEnumerator2 (Variables|Default|GetBeard) :NewEnumerator6 (Variables|Default|GetEyebrows) :NewEnumerator3 0 :NewEnumerator4 0 :NewEnumerator5 0) true false)))
          (:1
            (Class|SkinnedMeshComponent|SetSkeletalMesh (Variables|Default|GetTorso) (LocalVariables|GetL%20Mesh) true))
          (:2
            (Class|SkinnedMeshComponent|SetSkeletalMesh (Variables|Default|GetBottom) (LocalVariables|GetL%20Mesh) true))
          (:3
            (Class|SkinnedMeshComponent|SetSkeletalMesh (Variables|Default|GetFeet) (LocalVariables|GetL%20Mesh) true))))
      (:RowNotFound
        (switch int _array_index
          (:0
            (Class|SkinnedMeshComponent|SetSkeletalMesh (Variables|Default|GetHead) 0 true)
            (Development|SetHiddeninGame (Variables|Default|GetEyebrows) false false))
          (:1
            (Class|SkinnedMeshComponent|SetSkeletalMesh (Variables|Default|GetTorso) 0 true))
          (:2
            (Class|SkinnedMeshComponent|SetSkeletalMesh (Variables|Default|GetBottom) 0 true))
          (:3
            (Class|SkinnedMeshComponent|SetSkeletalMesh (Variables|Default|GetFeet) 0 true)))))))